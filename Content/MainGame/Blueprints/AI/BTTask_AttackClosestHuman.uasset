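; Behavior tree task that makes a zombie attack the closest human.
; It reads the ClosestHuman target from the zombie AI controller's blackboard and calls AttackCharacter on the controlled character.
; The attack result is written to the bAlreadyAttacked key and returned as the task's success.
; Any failed cast of controller, pawn or target fails the task.
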(event EventReceiveExecuteAI
  (params (OwnerController :type AI%20Controller%20Object%20Reference) (ControlledPawn :type Pawn%20Object%20Reference))
  (bind _asbp_zombie_aicontroller (Utilities|Casting|CastToBP_ZombieAIController OwnerController)
    (:then
      (Variables|Default|SetMyBlackboard (AI|GetBlackboard _asbp_zombie_aicontroller))
      (bind _asbp_character_base (Utilities|Casting|CastToBP_CharacterBase ControlledPawn)
        (:then
          (bind _asbp_character_base_2 (Utilities|Casting|CastToBP_CharacterBase (AI|Components|Blackboard|GetValueasObject (Variables|Default|GetMyBlackboard) (Utilities|Name|MakeLiteralName "ClosestHuman")))
            (:then
              (bind _success (Default|AttackCharacter _asbp_character_base _asbp_character_base_2))
              (AI|Components|Blackboard|SetValueasBool (Variables|Default|GetMyBlackboard) (Utilities|Name|MakeLiteralName "bAlreadyAttacked") _success)
              (AI|BehaviorTree|FinishExecute _success))
            (:CastFailed
              (AI|BehaviorTree|FinishExecute false :!label _label))))
        (:CastFailed
          (goto _label))))
    (:CastFailed
      (goto _label))))