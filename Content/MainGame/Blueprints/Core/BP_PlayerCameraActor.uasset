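; BP_PlayerCameraActor is a player camera that pans and zooms on a spring arm in response to axis input.
; Forward and Right inputs move a desired location along world X and Y through ClampLocation, while Zoom adjusts a clamped target arm length.
; Tick eases the actor location and arm length toward those targets with interpolation.
; A BlockControls macro checks a player controller flag, though no shown input uses it.
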(event EventBeginPlay
  (bind _returnvalue (Transformation|GetActorLocation))
  (Class|PlayerCameraActor|SetBaseLocation _returnvalue)
  (Variables|Components|SetLocation_Desired _returnvalue)
  (Variables|Components|SetZoom_Desired (Variables|/Script/Engine.SpringArmComponent|GetTargetArmLength (Variables|Default|GetSpringArm))))

(event EventTick
  (params (DeltaSeconds :type Float%20%28single-precision%29))
  (Variables|/Script/Engine.SpringArmComponent|SetTargetArmLength (Variables|Default|GetSpringArm) (Math|Interpolation|FInterpTo (Variables|/Script/Engine.SpringArmComponent|GetTargetArmLength (Variables|Default|GetSpringArm)) (Variables|Components|GetZoom_Desired) DeltaSeconds 2.0))
  (Transformation|SetActorLocation (Math|Interpolation|VInterpTo (Transformation|GetActorLocation) (Variables|Components|GetLocation_Desired) DeltaSeconds 5.0) false false))

(event Input|AxisEvents|InputAxisInputAxis_Zoom
  (params (AxisValue :type Float%20%28single-precision%29))
  (Variables|Components|SetZoom_Desired (Math|Float|Clamp(Float) (+ (Variables|Components|GetZoom_Desired) (* AxisValue 5e+01)) 5.0 2e+03)))

(event Input|AxisEvents|InputAxisInputAxis_Forward
  (params (AxisValue :type Float%20%28single-precision%29))
  (bind _returnvalue (Class|PlayerCameraActor|ClampLocation (+ (Variables|Components|GetLocation_Desired) (Math|Vector|MakeVector (* AxisValue 2e+01) 0.0 0.0))))
  (Variables|Components|SetLocation_Desired _returnvalue))

(event Input|AxisEvents|InputAxisInputAxis_Right
  (params (AxisValue :type Float%20%28single-precision%29))
  (bind _returnvalue (Class|PlayerCameraActor|ClampLocation (+ (Variables|Components|GetLocation_Desired) (Math|Vector|MakeVector 0.0 (* AxisValue 2e+01) 0.0))))
  (Variables|Components|SetLocation_Desired _returnvalue))

(fn ConstructionScript)

(fn SetDesiredLocation
  (params (NewLocation :type Vector)))