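; MyGridOutlinePainter is a grid outline painter that picks outline colors for grid cells marked as movable or attackable.
; GetColors checks each grid's gameplay tags for exact movable and attackable matches and returns every matching color, so a cell can carry both.
; GetColorPriority returns the color ordering, with the movable color listed before the attackable one.
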(fn GetColors
  (params (Grid :type Grid%20Object%20Reference))
  (bind _gridinfo (Variables|/Script/GridRuntime.Grid|GetGridInfo Grid))
  (bind _gameplaytags (Variables|/Script/GridRuntime.GridInfo|GetGameplayTags _gridinfo))
  (if (GameplayTags|HasTag _gameplaytags "(TagName=\"Grid.GridInfo.IsMovable\")" true)
    (Utilities|Array|Add (LocalVariables|GetRtn) (Variables|Default|GetMovableColor)))
  (if (GameplayTags|HasTag _gameplaytags "(TagName=\"Grid.GridInfo.IsAttackable\")" true)
    (Utilities|Array|Add (LocalVariables|GetRtn) (Variables|Default|GetAttackableColor)))
  (return (LocalVariables|GetRtn)))

(fn GetColorPriority
  (return (Utilities|Array|MakeArray (Variables|Default|GetMovableColor) (Variables|Default|GetAttackableColor))))