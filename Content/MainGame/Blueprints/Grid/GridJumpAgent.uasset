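; Grid movement agent that makes BP_CharacterBase pawns jump between grid positions at different heights.
; Check accepts height changes beyond a fixed threshold, capping upward jumps at the character's MaxJumpHeight while leaving drops uncapped.
; RequestMove launches the character with the velocity from its GetSuggestVelocity, failing if none is found.
; The character's jump-end event then unbinds itself and reports the move as completed successfully.
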(fn Check
  (params (Pawn :type Pawn%20Object%20Reference) (From :type Grid%20Object%20Reference) (To :type Grid%20Object%20Reference))
  (LocalVariables|SetDeltaHeight (- (Variables|/Script/GridRuntime.Grid|GetHeight To) (Variables|/Script/GridRuntime.Grid|GetHeight From)))
  (bind _astop_down_character (Utilities|Casting|CastToBP_CharacterBase Pawn)
    (:then
      (if (or (and (> (LocalVariables|GetDeltaHeight) 1e+04) (< (LocalVariables|GetDeltaHeight) (Variables|/Game/MainGame/Blueprints/Characters/BP_CharacterBase.BP_CharacterBase_C|GetMaxJumpHeight _astop_down_character))) (< (LocalVariables|GetDeltaHeight) -1e+04))
        (return true)
        (else
          _)))
    (:CastFailed
      _))
  (return false))

(fn RequestMove
  (params (Pawn :type Pawn%20Object%20Reference) (From :type Grid%20Object%20Reference) (To :type Grid%20Object%20Reference))
  (bind _astop_down_character (Utilities|Casting|CastToBP_CharacterBase Pawn)
    (:then
      (bind _output_get (LocalVariables|SetChar _astop_down_character))
      (bind (_succ _velocity) (Default|GetSuggestVelocity _output_get From To))
      (if _succ
        (Character|LaunchCharacter (LocalVariables|GetChar) _velocity false false)
        (EventDispatchers|BindEventtoJumpEndEvent (LocalVariables|GetChar) (EventDispatchers|CreateEvent :!event OnJumpEnd))
        (else
          (return false))))
    (:CastFailed
      (return false))))

(fn OnJumpEnd
  (params (Char :type BP%20Character%20Base%20Object%20Reference))
  (EventDispatchers|UnbindEventfromJumpEndEvent Char (EventDispatchers|CreateEvent :!event OnJumpEnd))
  (Default|CallOnMoveCompleted Char true))