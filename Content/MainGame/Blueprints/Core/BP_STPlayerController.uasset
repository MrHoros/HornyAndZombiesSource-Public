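; Player controller for a grid-based, turn-based tactics game, handling mouse input during Move and Attack phases and an Escape in-game menu.
; On phase changes it rebinds to the turn character's health and stamina events, refreshing the player GUI and attack options.
; Left click selects characters, double right click moves or attacks.
; Hovering grids previews pathfinding cost against stamina via a path guide, and hovering enemies shows hit chance.
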(event Custom|Reset
  ;[1 1 1] Escape keybind
  (Variables|Default|SetBlockControls false)
  (Widget|RemovefromParent (Variables|Default|GetMenu))
  (Variables|/Script/Engine.PlayerController|SetbShowMouseCursor self false)
  (Variables|Default|SetIsMenuClosed true))

(event Custom|OnTakeAnyDamage_Event_0
  (params (DamagedActor :type Actor%20Object%20Reference) (Damage :type Float%20%28single-precision%29) (DamageType :type Damage%20Type%20Object%20Reference) (InstigatedBy :type Controller%20Object%20Reference) (DamageCauser :type Actor%20Object%20Reference))
  ;[1 1 1] Update player gui health
  (if (and (== DamagedActor (Variables|Default|GetTurnCharacter)) (CallFunction|IsValidPhase))
    (Rendering|Components|TextRender|SetText (Variables|/Game/MainGame/UI/Widgets/CharacterInfo/Widget_PlayerGui.Widget_PlayerGui_C|GetCharacterHealth (Default|GetPlayerGui (Variables|Default|GetMyGameMode))) (Utilities|Text|ToText(Float) (Class|HealthComponent|GetHealth (Default|GetMyHealthComponent (Variables|Default|GetTurnCharacter))) "HalfToEven"))))

(event Custom|Dis_OnPhaseChanged_Event_0
  (params (OldPhase :type EPhase%20Enum :default "PE_None"))
  (if (CallFunction|IsValidPhase)
    (Utilities|IsValid (Variables|Default|GetTurnCharacter)
      (:Is%20Valid
        (EventDispatchers|UnbindEventfromOnStaminaChanged (Variables|Default|GetTurnCharacter) (delegate Custom|OnStaminaChanged_Event))
        (EventDispatchers|UnbindEventfromOnTakeAnyDamage (Variables|Default|GetTurnCharacter) (delegate Custom|OnTakeAnyDamage_Event_0)))
      (:Is%20Not%20Valid
        _))
    (Variables|Default|SetTurnCharacter (Default|GetCurrentTurnCharacter (Variables|Default|GetMyGameMode)))
    (CallFunction|UpdateScreenStatDisplayer)
    (EventDispatchers|AssignOnTakeAnyDamage (Variables|Default|GetTurnCharacter) (delegate Custom|OnTakeAnyDamage_Event_0))
    (EventDispatchers|AssignOnStaminaChanged (Variables|Default|GetTurnCharacter) (delegate Custom|OnStaminaChanged_Event))
    (if (Default|IsAITurn (Variables|Default|GetMyGameMode))
      (CallFunction|ClearPathGuide)
      (elif (Utilities|Enum|Equal(Enum) (Class|SmthTacticalGameModeBase|GetCurrentPhase (Variables|Default|GetMyGameMode)) "PE_Attack")
        (CallFunction|OnAttackPhase)))))

(event Custom|OnStaminaChanged_Event
  (params (NewStamina :type Integer))
  ;[1 1 1] Update player gui stamina
  (if (CallFunction|IsValidPhase)
    (Rendering|Components|TextRender|SetText (Variables|/Game/MainGame/UI/Widgets/CharacterInfo/Widget_PlayerGui.Widget_PlayerGui_C|GetCharacterStamina (Default|GetPlayerGui (Variables|Default|GetMyGameMode))) (Utilities|Text|ToText(Integer) NewStamina))))

(event EventBeginPlay
  (CallFunction|Setup)
  (EventDispatchers|AssignDisonPhaseChanged (Variables|Default|GetMyGameMode) (delegate Custom|Dis_OnPhaseChanged_Event_0)))

(event Input|ActionEvents|InputActionLeftClick
  (params (Key :type Key%20Structure :default "None"))
  ;[1 1 1] Left click
  (:Pressed
    (if (CallFunction|IsValidPhase)
      (Utilities|AreControlsBlocked
        (:False
          (if (not (Default|IsAITurn (Variables|Default|GetMyGameMode)))
            (CallFunction|HandleLeftClick)))))))

(event Input|ActionEvents|InputActionRightClick
  (params (Key :type Key%20Structure :default "None"))
  ;[1 1 1] Right click
  (:Pressed
    (if (CallFunction|IsValidPhase)
      (Utilities|AreControlsBlocked
        (:False
          (if (not (Default|IsAITurn (Variables|Default|GetMyGameMode)))
            (CallFunction|HandleRightClick)))))))

(event Input|AxisEvents|InputAxisMouseX
  (params (AxisValue :type Float%20%28single-precision%29))
  (bind _hitresult (Game|Player|GetHitResultUnderCursorbyChannel "TraceTypeQuery1" true))
  (bind (_bblockinghit _binitialoverlap _time _distance _location _impactpoint _normal _impactnormal _physmat _hitactor) (Collision|BreakHitResult _hitresult))
  ;[1 1 1] Mouse movement
  (if (CallFunction|IsValidPhase)
    (Utilities|AreControlsBlocked
      (:False
        (if (not (Default|IsAITurn (Variables|Default|GetMyGameMode)))
          (Utilities|IsValid (Variables|Default|GetMySelectedCharacter)
            (:Is%20Valid
              (Variables|Default|SetMouseHoverActor _hitactor)
              (Variables|Default|SetMouseHoverLocation _location)
              (Utilities|FlowControl|Sequence
                (:then_0
                  (CallFunction|HandleAttackChanceDisplayer))
                (:then_1
                  (bind _returnvalue (Class|GridManager|GetGridbyPosition (Default|GetGridManager (Variables|Default|GetMyGameMode)) (Variables|Default|GetMouseHoverLocation)))
                  (if (!= _returnvalue (Variables|Default|GetCursorOverGrid))
                    (Variables|Default|SetCursorOverGrid _returnvalue)
                    (CallFunction|OnCursorOverGridChanged)))))))))))

(event Input|AxisEvents|InputAxisMouseY
  (params (AxisValue :type Float%20%28single-precision%29))
  (bind _hitresult (Game|Player|GetHitResultUnderCursorbyChannel "TraceTypeQuery1" true))
  (bind (_bblockinghit _binitialoverlap _time _distance _location _impactpoint _normal _impactnormal _physmat _hitactor) (Collision|BreakHitResult _hitresult))
  ;[1 1 1] Mouse movement
  (if (CallFunction|IsValidPhase)
    (Utilities|AreControlsBlocked
      (:False
        (if (not (Default|IsAITurn (Variables|Default|GetMyGameMode)))
          (Utilities|IsValid (Variables|Default|GetMySelectedCharacter)
            (:Is%20Valid
              (Variables|Default|SetMouseHoverActor _hitactor)
              (Variables|Default|SetMouseHoverLocation _location)
              (Utilities|FlowControl|Sequence
                (:then_0
                  (CallFunction|HandleAttackChanceDisplayer))
                (:then_1
                  (bind _returnvalue (Class|GridManager|GetGridbyPosition (Default|GetGridManager (Variables|Default|GetMyGameMode)) (Variables|Default|GetMouseHoverLocation)))
                  (if (!= _returnvalue (Variables|Default|GetCursorOverGrid))
                    (Variables|Default|SetCursorOverGrid _returnvalue)
                    (CallFunction|OnCursorOverGridChanged)))))))))))

(event Input|KeyboardEvents|Escape
  (params (Key :type Key%20Structure :default "None"))
  ;[1 1 1] Escape keybind
  (:Pressed
    (if (CallFunction|IsValidPhase)
      (if (Variables|Default|GetIsMenuClosed)
        (Variables|Default|SetBlockControls true)
        (bind _returnvalue (UserInterface|CreateWidget "/Game/MainGame/UI/MenuInGame/MenuInGame.MenuInGame_C"))
        (bind _output_get (Variables|Default|SetMenu _returnvalue))
        (UserInterface|Viewport|AddtoViewport _output_get 1)
        (Variables|/Script/Engine.PlayerController|SetbShowMouseCursor self true)
        (Variables|Default|SetIsMenuClosed false)
        (else
          (Variables|Default|SetBlockControls false)
          (Widget|RemovefromParent (Variables|Default|GetMenu))
          (Variables|/Script/Engine.PlayerController|SetbShowMouseCursor self false)
          (Variables|Default|SetIsMenuClosed true))))))

(fn ConstructionScript
  (bind _asbp_gm (Utilities|Casting|CastToBP_GM (Game|GetGameMode)))
  (Variables|Default|SetMyGameMode _asbp_gm))

(fn OnCursorOverGridChanged
  (bind _myselectedcharacter (Variables|Default|GetMySelectedCharacter))
  (bind _pathguide (Variables|Default|GetPathGuide))
  (bind _pathguide_2 (Variables|Default|GetPathGuide))
  (bind _cursorovergrid (Variables|Default|GetCursorOverGrid))
  (bind _gridmanager (Variables|/Script/GridRuntime.Grid|GetGridManager _cursorovergrid))
  (Utilities|IsValid (Variables|Default|GetMySelectedCharacter)
    (:Is%20Valid
      (if (Default|IsCharacterTurn (Variables|Default|GetMyGameMode) (Variables|Default|GetMySelectedCharacter))
        (switch Utilities|FlowControl|Switch|SwitchonEPhase (Class|SmthTacticalGameModeBase|GetCurrentPhase (Variables|Default|GetMyGameMode))
          (:PE_Move
            (bind _returnvalue (Class|GridManager|GetGridbyPosition _gridmanager (Transformation|GetActorLocation (Variables|Default|GetMySelectedCharacter))))
            (bind _result (Class|GridUtilities|FindPath (Utilities|Struct|MakeGridPathfindingRequest (Variables|Default|GetMySelectedCharacter) _returnvalue (Variables|Default|GetCursorOverGrid)) (Class|GridManager|GetPathFinder _gridmanager)))
            (CallFunction|UpdateCurrentPathCost _result)
            (Math|Float|CompareFloat (Math|Conversions|ToFloat(Integer) (Variables|Default|GetCurrentPathCost)) (Math|Float|Max(Float) (Math|Conversions|ToFloat(Integer) (Class|STCharacterBase|GetStamina _myselectedcharacter)) (Class|STCharacterBase|GetAttackRange _myselectedcharacter))
              (:>
                (Class|PathGuide|SetDestinationDecalMaterial _pathguide "/Game/MainGame/Materials/M_GridHighlightedFail_Inst.M_GridHighlightedFail_Inst"))
              (:==
                (Class|PathGuide|SetDestinationDecalMaterial _pathguide "/Game/MainGame/Materials/M_GridHighlightedSuccess_Inst.M_GridHighlightedSuccess_Inst" :!label _label))
              (:<
                (goto _label)))
            (Class|PathGuide|SetPath (Variables|Default|GetPathGuide) _result)
            (Variables|Default|SetbShowMouseCursor true))
          (:PE_Attack
            (Class|PathGuide|Clear _pathguide_2 :!label _label_2)
            (Class|PathGuide|UpdateDecal _pathguide_2 (Utilities|Array|MakeArray (Transformation|GetActorLocation (Variables|Default|GetMySelectedCharacter)) (Class|Grid|GetCenter (Variables|Default|GetCursorOverGrid))))))
        (else
          (goto _label_2))))))

(fn UpdateCurrentPathCost
  (params (Path :type Array%20of%20Grid%20Object%20References))
  (bind _asmy_square_path_finder (Utilities|Casting|CastToMySquarePathFinder (Class|GridManager|GetPathFinder (Variables|Default|GetMyGridManager))))
  (Variables|Default|SetCurrentPathCost (Default|GetPathCost _asmy_square_path_finder Path)))

(fn HandleLeftClick
  (bind _hitresult (Game|Player|GetHitResultUnderCursorbyChannel "TraceTypeQuery1" true))
  (bind _myselectedcharacter (Variables|Default|GetMySelectedCharacter))
  (bind _myselectedcharacter_2 (Variables|Default|GetMySelectedCharacter))
  (bind (_bblockinghit _binitialoverlap _time _distance _location _impactpoint _normal _impactnormal _physmat _hitactor) (Collision|BreakHitResult _hitresult))
  (LocalVariables|SetHitLocation _location)
  (bind _output_get (LocalVariables|SetHitActor _hitactor))
  (Utilities|IsValid (Variables|Default|GetMySelectedCharacter)
    (:Is%20Valid
      (bind _asbp_character_base (Utilities|Casting|CastToBP_CharacterBase _output_get))
      (if (!= _asbp_character_base (Variables|Default|GetMySelectedCharacter))
        (CallFunction|HideStatDsiplayer)
        (Default|SelectCharacter (Variables|Default|GetMyGameMode) _asbp_character_base)
        (Default|RefreshAllGrids (Variables|Default|GetMyGridManager))
        (if (!= (Default|GetCurrentTurnCharacter (Variables|Default|GetMyGameMode)) (Variables|Default|GetMySelectedCharacter))
          (Default|UpdateStatDisplayer _myselectedcharacter)
          (bind _newparam (Default|GetWorldGui _myselectedcharacter))
          (Default|SetCanvasVisibleState _newparam "NewEnumerator1" "Visible"))
        (elif (== (Variables|Default|GetMySelectedCharacter) (Default|GetCurrentTurnCharacter (Variables|Default|GetMyGameMode)))
          (bind _newparam_2 (Default|GetWorldGui (Variables|Default|GetMySelectedCharacter)))
          (switch Utilities|FlowControl|Switch|SwitchonESlateVisibility (Widget|GetVisibility (Variables|/Game/MainGame/UI/Widgets/CharacterInfo/WidgetCharacterWorldGui.WidgetCharacterWorldGui_C|GetEndPhase _newparam_2))
            (:Visible
              (CallFunction|HideStatDsiplayer))
            (:Hidden
              (Default|SetCanvasVisibleState _newparam_2 "NewEnumerator0" "Visible" :!label _label)
              (if (and (Utilities|Enum|Equal(Enum) "PE_Attack" (Class|SmthTacticalGameModeBase|GetCurrentPhase (Variables|Default|GetMyGameMode))) (and (Utilities|Enum|Equal(Enum) (Default|GetAttackMode _myselectedcharacter_2) "NewEnumerator0") (Variables|/Game/MainGame/Blueprints/Characters/BP_CharacterBase.BP_CharacterBase_C|GetHasAbility _myselectedcharacter_2)))
                (Default|SetCanvasVisibleState _newparam_2 "NewEnumerator3" "Visible")))
            (:HitTestInvisible
              (goto _label))
            (:SelfHitTestInvisible
              (goto _label))))))))

(fn HandleRightClick
  (bind _hitresult (Game|Player|GetHitResultUnderCursorbyChannel "TraceTypeQuery1" true))
  (bind _myselectedcharacter (Variables|Default|GetMySelectedCharacter))
  (bind (_bblockinghit _binitialoverlap _time _distance _location _impactpoint _normal _impactnormal _physmat _hitactor) (Collision|BreakHitResult _hitresult))
  (LocalVariables|SetHitLocation _location)
  (LocalVariables|SetHitActor _hitactor)
  (Utilities|IsValid _myselectedcharacter
    (:Is%20Valid
      (if (Default|IsCharacterTurn (Variables|Default|GetMyGameMode) _myselectedcharacter)
        (CallFunction|HideStatDsiplayer)
        (switch Utilities|FlowControl|Switch|SwitchonEPhase (Class|SmthTacticalGameModeBase|GetCurrentPhase (Variables|Default|GetMyGameMode))
          (:PE_Move
            ;[1 1 1] On right click ( move phase )
            (if (Variables|Default|GetMoveDebounce)
              (bind _success (CallFunction|TryMovetoHitLocation (LocalVariables|GetHitLocation)))
              (if _success
                (Default|SelectCharacter (Variables|Default|GetMyGameMode))
                (CallFunction|ClearPathGuide)
                (Variables|Default|SetMoveDebounce false)
                (else
                  (Variables|Default|SetMoveDebounce false)))
              (else
                (Variables|Default|SetMoveDebounce true))))
          (:PE_Attack
            (if (Variables|Default|GetAttackDebounce)
              (switch Utilities|FlowControl|Switch|SwitchonAttackModeEnum (Default|GetAttackMode (Variables|Default|GetMySelectedCharacter))
                (:NewEnumerator0
                  ;[1 1 1] On right click ( attack phase )
                  (bind _asbp_character_base (Utilities|Casting|CastToBP_CharacterBase (LocalVariables|GetHitActor))
                    (:then
                      (bind _output_get (LocalVariables|SetHitCharacter _asbp_character_base))
                      (bind _success_2 (Default|AttackCharacter (Variables|Default|GetTurnCharacter) _output_get))
                      (if _success_2
                        (Default|SelectCharacter (Variables|Default|GetMyGameMode))
                        (CallFunction|ClearPathGuide)
                        (else
                          (Variables|Default|SetAttackDebounce false))))
                    (:CastFailed
                      (Variables|Default|SetAttackDebounce false))))
                (:NewEnumerator1
                  (Default|OnAbilityRightClickedActor (Variables|Default|GetMySelectedCharacter) (LocalVariables|GetHitActor))))
              (else
                (Variables|Default|SetAttackDebounce true)))))))))

(fn UpdateScreenStatDisplayer
  (LocalVariables|SetPlayerGui (Default|GetPlayerGui (Variables|Default|GetMyGameMode)))
  (Utilities|FlowControl|Sequence
    (:then_0
      ;[1 1 1] Damage
      (Rendering|Components|TextRender|SetText (Variables|/Game/MainGame/UI/Widgets/CharacterInfo/Widget_PlayerGui.Widget_PlayerGui_C|GetCharacterDamage (LocalVariables|GetPlayerGui)) (Utilities|Text|ToText(Integer) (Class|STCharacterBase|GetDamage (Variables|Default|GetTurnCharacter)))))
    (:then_1
      ;[1 1 1] Health
      (Rendering|Components|TextRender|SetText (Variables|/Game/MainGame/UI/Widgets/CharacterInfo/Widget_PlayerGui.Widget_PlayerGui_C|GetCharacterHealth (LocalVariables|GetPlayerGui)) (Utilities|Text|ToText(Float) (Class|HealthComponent|GetHealth (Default|GetMyHealthComponent (Variables|Default|GetTurnCharacter))) "HalfToEven")))
    (:then_2
      ;[1 1 1] Stamina
      (Rendering|Components|TextRender|SetText (Variables|/Game/MainGame/UI/Widgets/CharacterInfo/Widget_PlayerGui.Widget_PlayerGui_C|GetCharacterStamina (LocalVariables|GetPlayerGui)) (Utilities|Text|ToText(Integer) (Class|STCharacterBase|GetStamina (Variables|Default|GetTurnCharacter)))))
    (:then_3
      ;[1 1 1] Character name
      (Rendering|Components|TextRender|SetText (Variables|/Game/MainGame/UI/Widgets/CharacterInfo/Widget_PlayerGui.Widget_PlayerGui_C|GetCharacterName (LocalVariables|GetPlayerGui)) (Utilities|Text|ToText(String) (Class|STCharacterBase|GetUnitName (Variables|Default|GetTurnCharacter)))))
    (:then_4
      ;[1 1 1] Attack range
      (Rendering|Components|TextRender|SetText (Variables|/Game/MainGame/UI/Widgets/CharacterInfo/Widget_PlayerGui.Widget_PlayerGui_C|GetCharacterAttackRange (LocalVariables|GetPlayerGui)) (Utilities|Text|ToText(Float) (Class|STCharacterBase|GetAttackRange (Variables|Default|GetTurnCharacter)) "HalfToEven")))
    (:then_5
      ;[1 1 1] Mod
      (Rendering|Components|TextRender|SetText (Variables|/Game/MainGame/UI/Widgets/CharacterInfo/Widget_PlayerGui.Widget_PlayerGui_C|GetCharacterMod (LocalVariables|GetPlayerGui)) (Utilities|Text|ToText(Integer) (Class|STCharacterBase|GetModPoints (Variables|Default|GetTurnCharacter)))))
    (:then_6
      ;[1 1 1] Ach
      (Rendering|Components|TextRender|SetText (Variables|/Game/MainGame/UI/Widgets/CharacterInfo/Widget_PlayerGui.Widget_PlayerGui_C|GetCharacterAttackBoost (LocalVariables|GetPlayerGui)) (Utilities|Text|FormatText "+{Integer}%" (Class|STCharacterBase|GetAttackChanceBoost (Variables|Default|GetTurnCharacter)))))
    (:then_7
      ;[1 1 1] Dch
      (Rendering|Components|TextRender|SetText (Variables|/Game/MainGame/UI/Widgets/CharacterInfo/Widget_PlayerGui.Widget_PlayerGui_C|GetCharacterDefenseBoost (LocalVariables|GetPlayerGui)) (Utilities|Text|FormatText "+{Integer}%" (Class|STCharacterBase|GetDefenseChanceBoost (Variables|Default|GetTurnCharacter)))))
    (:then_8
      ;[1 1 1] Team name
      (Rendering|Components|TextRender|SetText (Variables|/Game/MainGame/UI/Widgets/CharacterInfo/Widget_PlayerGui.Widget_PlayerGui_C|GetCharacterTeam (LocalVariables|GetPlayerGui)) (Utilities|Text|ToText(String) (Class|STCharacterBase|GetTeamName (Variables|Default|GetTurnCharacter)))))
    (:then_9
      ;[1 0.9796 0.5782] Colors
      (Appearance|SetColorandOpacity (Variables|/Game/MainGame/UI/Widgets/CharacterInfo/Widget_PlayerGui.Widget_PlayerGui_C|GetCharacterTeam (LocalVariables|GetPlayerGui)) (Utilities|Struct|MakeSlateColor (Math|Conversions|ToLinearColor(Color) (Class|STCharacterBase|GetTeamColor (Variables|Default|GetTurnCharacter))) (.ColorUseRule (Utilities|Struct|BreakSlateColor (Variables|/Script/UMG.TextBlock|GetColorAndOpacity (Variables|/Game/MainGame/UI/Widgets/CharacterInfo/Widget_PlayerGui.Widget_PlayerGui_C|GetCharacterTeam (LocalVariables|GetPlayerGui)))))) :!class /Script/UMG.TextBlock)
      (Appearance|SetColorandOpacity (Variables|/Game/MainGame/UI/Widgets/CharacterInfo/Widget_PlayerGui.Widget_PlayerGui_C|GetCharacterName (LocalVariables|GetPlayerGui)) (Utilities|Struct|MakeSlateColor (Math|Conversions|ToLinearColor(Color) (Class|STCharacterBase|GetTeamColor (Variables|Default|GetTurnCharacter))) (.ColorUseRule (Utilities|Struct|BreakSlateColor (Variables|/Script/UMG.TextBlock|GetColorAndOpacity (Variables|/Game/MainGame/UI/Widgets/CharacterInfo/Widget_PlayerGui.Widget_PlayerGui_C|GetCharacterTeam (LocalVariables|GetPlayerGui)))))) :!class /Script/UMG.TextBlock))))

(fn HideStatDsiplayer
  (bind _newparam (Default|GetWorldGui (Variables|Default|GetMySelectedCharacter)))
  (Default|SetAllCanvasVisibleState _newparam "Hidden"))

(fn GetCharacterHealthComponent
  (params (Character :type BP%20Character%20Base%20Object%20Reference))
  (return (Default|GetMyHealthComponent Character)))

(fn ClearPathGuide
  (Class|PathGuide|SetPath (Variables|Default|GetPathGuide) (LocalVariables|GetEmptyPath)))

(fn TryMovetoHitLocation
  (params (HitLocation :type Vector))
  (bind _currentpathcost (Variables|Default|GetCurrentPathCost))
  (LocalVariables|SetMoveLocation HitLocation)
  (bind _result (Utilities|NegateInt (Math|Integer|Absolute(Integer) _currentpathcost))
    (:%20%20
      (if (<= _currentpathcost (Class|STCharacterBase|GetStamina (Default|GetSelectedCharacter (Variables|Default|GetMyGameMode))))
        (Class|STCharacterBase|ChangeStamina (Variables|Default|GetMySelectedCharacter) _result)
        (bind _success (Default|MoveSelectedCharactertoLocation (Variables|Default|GetMyGameMode) (LocalVariables|GetMoveLocation)))
        (return _success)
        (else
          (return false))))))

(fn OnArrivalGoal
  (Variables|Default|SetMoveDebounce false))

(fn HandleAttackChanceDisplayer
  (bind _mousehoveractor (Variables|Default|GetMouseHoverActor))
  (Utilities|IsValid _mousehoveractor
    (:Is%20Valid
      (if (and (!= _mousehoveractor (Variables|Default|GetMySelectedCharacter)) (!= (Variables|Default|GetMouseHoverActor) (Variables|Default|GetLastMouseHoveredCharacter)))
        (Utilities|IsValid (Variables|Default|GetLastMouseHoveredCharacter)
          (:Is%20Valid
            (bind _asbp_character_base (Utilities|Casting|CastToBP_CharacterBase (Variables|Default|GetLastMouseHoveredCharacter)))
            (bind _aswidget_character_world_gui (Utilities|Casting|CastToWidgetCharacterWorldGui (UserInterface|GetWidget (Variables|/Game/MainGame/Blueprints/Characters/BP_CharacterBase.BP_CharacterBase_C|GetWorldInfoGui _asbp_character_base))))
            (Default|SetCanvasVisibleState _aswidget_character_world_gui "NewEnumerator2" "Hidden")
            (Variables|Default|SetLastMouseHoveredCharacter 0))
          (:Is%20Not%20Valid
            _))
        (bind _asstcharacter_base (Utilities|Casting|CastToSTCharacterBase (Variables|Default|GetMouseHoverActor)))
        (if (!= (Class|STCharacterBase|GetTeamIndex _asstcharacter_base) (Class|STCharacterBase|GetTeamIndex (Variables|Default|GetMySelectedCharacter)))
          (bind _asbp_character_base_2 (Utilities|Casting|CastToBP_CharacterBase (Variables|Default|GetMouseHoverActor)))
          (bind _aswidget_character_world_gui_2 (Utilities|Casting|CastToWidgetCharacterWorldGui (UserInterface|GetWidget (Variables|/Game/MainGame/Blueprints/Characters/BP_CharacterBase.BP_CharacterBase_C|GetWorldInfoGui _asbp_character_base_2))))
          (Default|SetAttackChanceText _aswidget_character_world_gui_2 (Class|STCharacterBase|GetChancetoAttackCharacter (Variables|Default|GetMySelectedCharacter) _asbp_character_base_2))
          (Default|SetCanvasVisibleState _aswidget_character_world_gui_2 "NewEnumerator2" "HitTestInvisible")
          (Variables|Default|SetLastMouseHoveredCharacter (Variables|Default|GetMouseHoverActor)))))))

(fn Setup
  (Utilities|FlowControl|Sequence
    (:then_0
      (Variables|Default|SetMyGridManager (Default|GetGridManager (Variables|Default|GetMyGameMode))))
    (:then_1
      (bind _returnvalue (Game|SpawnActorfromClass "/Game/MainGame/Blueprints/Grid/MyPathGuide.MyPathGuide_C" (Math|Transform|MakeTransform "0, 0, 0") "AlwaysSpawn" 0 0))
      (Variables|Default|SetPathGuide _returnvalue)
      (Game|GetCurrentLevelName true)
      (Class|PathGuide|SetStartDecalMaterial (Variables|Default|GetPathGuide) "/Game/MainGame/Materials/M_GridStartPosition_Inst.M_GridStartPosition_Inst")
      (Class|PathGuide|SetDestinationDecalMaterial (Variables|Default|GetPathGuide) "/Game/MainGame/Materials/M_GridHighlightedSuccess_Inst.M_GridHighlightedSuccess_Inst"))))

(fn OnAttackPhase
  (bind _turncharacter (Variables|Default|GetTurnCharacter))
  (bind _turncharacter_2 (Variables|Default|GetTurnCharacter))
  (bind _aswidget_character_world_gui (Utilities|Casting|CastToWidgetCharacterWorldGui (UserInterface|GetWidget (Variables|/Game/MainGame/Blueprints/Characters/BP_CharacterBase.BP_CharacterBase_C|GetWorldInfoGui (Variables|Default|GetTurnCharacter)))))
  (bind _output_get (LocalVariables|SetTurnCharacterWidget _aswidget_character_world_gui))
  (Default|SetCanvasVisibleState _output_get "NewEnumerator0" "Visible")
  (if (and (Utilities|Enum|Equal(Enum) (Default|GetAttackMode _turncharacter_2) "NewEnumerator0") (Variables|/Game/MainGame/Blueprints/Characters/BP_CharacterBase.BP_CharacterBase_C|GetHasAbility _turncharacter_2))
    (Default|SetCanvasVisibleState (LocalVariables|GetTurnCharacterWidget) "NewEnumerator3" "Visible")
    (Math|Integer|CompareInt (Class|STCharacterBase|GetModPoints _turncharacter) (Variables|/Game/MainGame/Blueprints/Characters/BP_CharacterBase.BP_CharacterBase_C|GetAbilityCost _turncharacter)
      (:>
        (Default|SetAbilityAvailability (LocalVariables|GetTurnCharacterWidget) true :!label _label))
      (:==
        (goto _label))
      (:<
        (Default|SetAbilityAvailability (LocalVariables|GetTurnCharacterWidget) false)))))

(fn IsValidPhase
  (switch Utilities|FlowControl|Switch|SwitchonEPhase (Class|SmthTacticalGameModeBase|GetCurrentPhase (Variables|Default|GetMyGameMode))
    (:PE_None
      _)
    (:PE_Init
      _)
    (:PE_Setup
      _)
    (:PE_Move
      (return true))
    (:PE_Attack
      (return true))
    (:PE_TurnEnd
      _)
    (:PE_LevelEnd
      _))
  (return false))