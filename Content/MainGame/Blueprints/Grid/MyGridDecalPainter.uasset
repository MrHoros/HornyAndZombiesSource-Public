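; Grid decal painter that picks the decal material for each square grid cell, showing movable, attackable or normal state.
; GetDecalMaterial caches the square material set as current, then checks the cell's gameplay tags, with movable taking priority over attackable.
; Setter functions swap the attackable material at runtime or restore its default.
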(fn GetDecalMaterial
  (params (Grid :type Grid%20Object%20Reference))
  (bind _gridinfo (Variables|/Script/GridRuntime.Grid|GetGridInfo Grid))
  (bind _gameplaytags (Variables|/Script/GridRuntime.GridInfo|GetGameplayTags _gridinfo))
  (Utilities|Casting|CastToSquareGrid Grid)
  ;[1 1 1] Setup square decal material
  (Variables|Default|SetCurrNormalDecalMat (Variables|Default|GetSquareNormalDecalMat))
  (Variables|Default|SetCurrMovableDecalMat (Variables|Default|GetSquareMovableDecalMat))
  (Variables|Default|SetCurrAttackableDecalMat (Variables|Default|GetSquareAttackableDecalMat))
  (Variables|Default|SetCurrHighlightedDecalMat (Variables|Default|GetSquareHighlightedDecalMat))
  ;[1 1 1] Movable material's priority is higher than attackable
  (if (GameplayTags|HasTag _gameplaytags "(TagName=\"Grid.GridInfo.IsMovable\")" true)
    (return (Variables|Default|GetCurrMovableDecalMat))
    (elif (GameplayTags|HasTag _gameplaytags "(TagName=\"Grid.GridInfo.IsAttackable\")" true)
      (return (Variables|Default|GetCurrAttackableDecalMat))
      (else
        (return (Variables|Default|GetCurrNormalDecalMat))))))

(fn SetSquareAttackableMaterial
  (params (NewMaterial :type Material%20Interface%20Object%20Reference))
  (Utilities|IsValid NewMaterial
    (:Is%20Valid
      (Variables|Default|SetSquareAttackableDecalMat NewMaterial)
      (return))))

(fn SetDefaultAttackableMaterial
  (Variables|Default|SetSquareAttackableDecalMat (Variables|Default|GetDefaultSquareAttackableDecalMat))
  (return))