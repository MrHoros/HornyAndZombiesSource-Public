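; Grid manager for turn-based tactics that shows where the selected character can move or attack, based on the current phase.
; Movable cells come from stamina-limited pathfinding; attackable cells from a circular range query plus sight checks.
; Gameplay tags mark both sets, so clearing one keeps shared cells visible.
; It also picks the cell scoring highest on summed distance from a team, though its reachability "penalty" actually raises the score.
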(event EventBeginPlay
  (bind _asbp_gm (Utilities|Casting|CastToBP_GM (Game|GetGameMode)))
  (Variables|Default|SetMyGameMode _asbp_gm))

(event Collision|EventActorBeginOverlap
  (params (OtherActor :type Actor%20Object%20Reference)))

(event EventTick
  (params (DeltaSeconds :type Float%20%28single-precision%29)))

(fn ConstructionScript)

(fn ClearAttackableGrids
  (bind _attackablegrids (Variables|Default|GetAttackableGrids))
  (for _array_element _attackablegrids
    (GameplayTags|RemoveGameplayTag (Variables|/Script/GridRuntime.GridInfo|GetGameplayTags (Variables|/Script/GridRuntime.Grid|GetGridInfo _array_element)) "(TagName=\"Grid.GridInfo.IsAttackable\")" :!class /Script/GameplayTags.BlueprintGameplayTagLibrary)
    (Class|GridInfo|Dirty (Variables|/Script/GridRuntime.Grid|GetGridInfo _array_element))
    (if (not (GameplayTags|HasTag (Variables|/Script/GridRuntime.GridInfo|GetGameplayTags (Variables|/Script/GridRuntime.Grid|GetGridInfo _array_element)) "(TagName=\"Grid.GridInfo.IsMovable\")" true))
      (Class|Grid|SetVisibility _array_element false)))
  (Utilities|Array|Clear _attackablegrids))

(fn ClearMovableGrids
  (bind _movablegrids (Variables|Default|GetMovableGrids))
  (for _array_element _movablegrids
    (GameplayTags|RemoveGameplayTag (Variables|/Script/GridRuntime.GridInfo|GetGameplayTags (Variables|/Script/GridRuntime.Grid|GetGridInfo _array_element)) "(TagName=\"Grid.GridInfo.IsMovable\")" :!class /Script/GameplayTags.BlueprintGameplayTagLibrary)
    (Class|GridInfo|Dirty (Variables|/Script/GridRuntime.Grid|GetGridInfo _array_element))
    (if (not (GameplayTags|HasTag (Variables|/Script/GridRuntime.GridInfo|GetGameplayTags (Variables|/Script/GridRuntime.Grid|GetGridInfo _array_element)) "(TagName=\"Grid.GridInfo.IsAttackable\")" true))
      (Class|Grid|SetVisibility _array_element false)))
  (Utilities|Array|Clear _movablegrids))

(fn GetGridsbyRangeFloat
  (params (Start%20location :type Vector) (Range :type Float%20%28single-precision%29))
  (LocalVariables|SetMyRange Range)
  (LocalVariables|SetStartLocation Start%20location)
  (LocalVariables|SetGridsInRange (Utilities|Array|MakeArray))
  (if (> (LocalVariables|GetMyRange) 0.0)
    (bind _returnvalue (Class|SquareGridManager|GetSquareGridbyPosition (LocalVariables|GetStartLocation)))
    (LocalVariables|SetMyCenter (Class|Grid|GetCenter _returnvalue))
    (bind _grids (Class|SquareGridManager|GetSquareGridsbyRange _returnvalue (+ (Math|Float|Truncate (LocalVariables|GetMyRange)) 1) true))
    (for _array_element _grids
      (if (<= (Math|Vector|Distance(Vector) (LocalVariables|GetMyCenter) (Class|Grid|GetCenter _array_element)) (* (LocalVariables|GetMyRange) 1e+02))
        (Utilities|Array|Add (LocalVariables|GetGridsInRange) _array_element)))
    (return (LocalVariables|GetGridsInRange))
    (else
      (return (LocalVariables|GetGridsInRange)))))

(fn UpdateMovableGrid
  (params (NewVisibility :type Boolean))
  (LocalVariables|SetSelectedCharacter (Default|GetSelectedCharacter (Variables|Default|GetMyGameMode)))
  (CallFunction|ClearMovableGrids)
  (if NewVisibility
    (Utilities|IsValid (LocalVariables|GetSelectedCharacter)
      (:Is%20Valid
        (bind _result (Class|GridUtilities|GetReachableGrids (LocalVariables|GetSelectedCharacter) (Math|Conversions|ToFloat(Integer) (Class|STCharacterBase|GetStamina (LocalVariables|GetSelectedCharacter))) (Class|GridManager|GetPathFinder)))
        (bind _output_get (Variables|Default|SetMovableGrids _result))
        (for _array_element _output_get
          (Class|Grid|SetVisibility _array_element true)
          (GameplayTags|AddGameplayTag (Variables|/Script/GridRuntime.GridInfo|GetGameplayTags (Variables|/Script/GridRuntime.Grid|GetGridInfo _array_element)) "(TagName=\"Grid.GridInfo.IsMovable\")" :!class /Script/GameplayTags.BlueprintGameplayTagLibrary)
          (Class|GridInfo|Dirty (Variables|/Script/GridRuntime.Grid|GetGridInfo _array_element)))))))

(fn UpdateAttackableGrid
  (params (NewVisibility :type Boolean))
  (LocalVariables|SetSelectedCharacter (Default|GetSelectedCharacter (Variables|Default|GetMyGameMode)))
  (CallFunction|ClearAttackableGrids)
  (if NewVisibility
    (Utilities|IsValid (LocalVariables|GetSelectedCharacter)
      (:Is%20Valid
        (bind _grids (CallFunction|GetGridsbyRangeFloat (Transformation|GetActorLocation (LocalVariables|GetSelectedCharacter)) (Default|GetMaxCostinCurrentPhase (LocalVariables|GetSelectedCharacter))))
        (bind _output_get (Variables|Default|SetAttackableGrids _grids))
        (for _array_element _output_get
          (if (and (Utilities|Enum|Equal(Enum) (Class|SmthTacticalGameModeBase|GetCurrentPhase (Variables|Default|GetMyGameMode)) "PE_Attack") (Default|IsGridCharacterinSight (LocalVariables|GetSelectedCharacter) _array_element))
            (Class|Grid|SetVisibility _array_element true)
            (GameplayTags|AddGameplayTag (Variables|/Script/GridRuntime.GridInfo|GetGameplayTags (Variables|/Script/GridRuntime.Grid|GetGridInfo _array_element)) "(TagName=\"Grid.GridInfo.IsAttackable\")" :!class /Script/GameplayTags.BlueprintGameplayTagLibrary)
            (Class|GridInfo|Dirty (Variables|/Script/GridRuntime.Grid|GetGridInfo _array_element))))))))

(fn RefreshAllGrids
  (Default|CallDisRefreshGridOccupiers)
  (switch Utilities|FlowControl|Switch|SwitchonEPhase (Class|SmthTacticalGameModeBase|GetCurrentPhase (Variables|Default|GetMyGameMode))
    (:PE_Move
      (CallFunction|UpdateMovableGrid true)
      (CallFunction|UpdateAttackableGrid false))
    (:PE_Attack
      (CallFunction|UpdateMovableGrid false)
      (CallFunction|UpdateAttackableGrid true))))

(fn GetFurthestGridfromTeamCharacters
  (params (TeamIndex :type Integer) (ReachableGrids :type Array%20of%20Grid%20Object%20References))
  (bind _gridmap (LocalVariables|GetGridMap))
  (LocalVariables|SetEnemyCharacters (Class|SmthTacticalGameModeBase|GetCharactersOfTeamIndex (Variables|Default|GetMyGameMode) TeamIndex))
  (for _array_element ReachableGrids
    ;[1 1 1] Calculate each grid value based on distances and enemy reachable grids
    (for _array_element_2 (LocalVariables|GetEnemyCharacters)
      (bind _asbp_character_base (Utilities|Casting|CastToBP_CharacterBase _array_element_2))
      (LocalVariables|SetTotalDistance (+ (Math|Vector|Distance(Vector) (Transformation|GetActorLocation _array_element_2) (Class|Grid|GetCenter _array_element)) (LocalVariables|GetTotalDistance)))
      (bind _result (Class|GridUtilities|GetReachableGrids _asbp_character_base (Math|Conversions|ToFloat(Integer) (Class|STCharacterBase|GetMaxStamina _asbp_character_base)) (Class|GridManager|GetPathFinder)))
      ;;[1 1 1] Penalty for being in the attack range
      (if (>= (Utilities|Array|FindItem _result _array_element) 0)
        (LocalVariables|SetTotalDistance (+ 1e+01 (LocalVariables|GetTotalDistance)))))
    (Utilities|Map|Add (LocalVariables|GetGridMap) _array_element (LocalVariables|GetTotalDistance))
    (LocalVariables|SetTotalDistance 0.0))
  (Utilities|FlowControl|Sequence
    (:then_0
      ;[1 0.9101 0.5277] [DEBUG] draw strings
      (if (LocalVariables|GetbDebugMode)
        (bind _values (Utilities|Map|Values _gridmap))
        (bind _keys (Utilities|Map|Keys _gridmap))
        (for _index (range 0 (- (Utilities|Map|Length (LocalVariables|GetGridMap)) 1))
          (Rendering|Debug|DrawDebugString (Class|Grid|GetCenter (Utilities|Array|Get(acopy) _keys _index)) (Utilities|String|ToString(Integer) (Math|Float|Truncate (Utilities|Array|Get(acopy) _values _index))) 0 (Math|Conversions|ToLinearColor(Float) (Utilities|Array|Get(acopy) _values _index)) 4.0))))
    (:then_1
      ;[1 1 1] Return best spot (grid with the highest calculated value)
      (bind _values_2 (Utilities|Map|Values (LocalVariables|GetGridMap)))
      (bind _keys_2 (Utilities|Map|Keys (LocalVariables|GetGridMap)))
      (return (Utilities|Array|Get(acopy) _keys_2 (.IndexOfMaxValue (Math|Float|MaxOfFloatArray _values_2)))))))