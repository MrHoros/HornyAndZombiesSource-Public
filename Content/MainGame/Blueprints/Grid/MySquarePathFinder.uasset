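; A square-grid pathfinder that decides which tiles a requesting character can reach and what a path costs.
; IsReachable extends the parent check by requiring a BP_CharacterBase sender and an unoccupied MyGridInfo destination.
; It also asks the character's game mode to reject destinations with another character over them.
; GetPathCost totals the step cost between each consecutive pair of grids in the path.
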(fn IsReachable
  (params (Start :type Grid%20Object%20Reference) (Dest :type Grid%20Object%20Reference))
  (LocalVariables|SetStartGrid Start)
  (bind _output_get (LocalVariables|SetDestinationGrid Dest))
  (bind _returnvalue (|CallParentFunction (LocalVariables|GetStartGrid) _output_get))
  (if _returnvalue
    (bind _asbp_character_base (Utilities|Casting|CastToBP_CharacterBase (.Sender (Utilities|Struct|BreakGridPathfindingRequest (Variables|Default|GetRequest))))
      (:then
        (bind _output_get_2 (LocalVariables|SetCharacter _asbp_character_base))
        (LocalVariables|SetGamemode (Variables|/Game/MainGame/Blueprints/Characters/BP_CharacterBase.BP_CharacterBase_C|GetMyGamemode _output_get_2))
        (bind _asmy_grid_info (Utilities|Casting|CastToMyGridInfo (Variables|/Script/GridRuntime.Grid|GetGridInfo (LocalVariables|GetDestinationGrid)))
          (:then
            (bind _isoccupied (Default|GetIsOccupied _asmy_grid_info))
            (if (not _isoccupied)
              (Utilities|IsValid (Default|GetCharacterOverGrid (LocalVariables|GetGamemode) (LocalVariables|GetDestinationGrid) (Utilities|Array|MakeArray))
                (:Is%20Valid
                  _)
                (:Is%20Not%20Valid
                  (return true)))))
          (:CastFailed
            _)))
      (:CastFailed
        _)))
  (return false))

(fn GetPathCost
  (params (Path :type Array%20of%20Grid%20Object%20References))
  (LocalVariables|SetMyPath Path)
  (LocalVariables|SetPathCost 0)
  (for _index (range 0 (- (Utilities|Array|LastIndex Path) 1))
    (bind _output_get (LocalVariables|SetcurrentIndex _index))
    (Math|Integer|IncrementInt _output_get
      (:%20%20
        (bind _returnvalue (Class|GridPathFinder|GetCost (Utilities|Array|Get(acopy) (LocalVariables|GetMyPath) (- (LocalVariables|GetCurrentIndex) 1)) (Utilities|Array|Get(acopy) (LocalVariables|GetMyPath) (LocalVariables|GetCurrentIndex))))
        (LocalVariables|SetPathCost (+ _returnvalue (LocalVariables|GetPathCost))))))
  (return (LocalVariables|GetPathCost)))