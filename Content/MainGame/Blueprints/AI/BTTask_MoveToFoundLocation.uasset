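; Behavior tree task that moves a zombie AI's character to the location stored in the blackboard's MoveLocation key.
; It casts the controller and pawn, then delegates the move to the game mode's MoveCharacterToLocation.
; The returned result is written to the bAlreadyMoved key and finishes the task as success or failure, with an optional debug sphere at the target.
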(event EventReceiveExecuteAI
  (params (OwnerController :type AI%20Controller%20Object%20Reference) (ControlledPawn :type Pawn%20Object%20Reference))
  (bind _asbp_zombie_aicontroller (Utilities|Casting|CastToBP_ZombieAIController OwnerController)
    (:then
      (Variables|Default|SetMyAIController _asbp_zombie_aicontroller)
      (bind _asbp_character_base (Utilities|Casting|CastToBP_CharacterBase ControlledPawn)
        (:then
          (Variables|Default|SetMyCharacter _asbp_character_base)
          (bind _asbp_gm (Utilities|Casting|CastToBP_GM (Game|GetGameMode)))
          (bind _success (Default|MoveCharactertoLocation _asbp_gm (AI|Components|Blackboard|GetValueasVector (AI|GetBlackboard (Variables|Default|GetMyAIController)) (Utilities|Name|MakeLiteralName "MoveLocation")) (Variables|Default|GetMyCharacter)))
          (if (Variables|Default|GetbDebugMode)
            (Rendering|Debug|DrawDebugSphere (AI|Components|Blackboard|GetValueasVector (AI|GetBlackboard (Variables|Default|GetMyAIController)) (Utilities|Name|MakeLiteralName "MoveLocation")) 4e+01 12 "(R=1.000000,G=0.131786,B=0.000000,A=1.000000)" 4.0))
          (AI|Components|Blackboard|SetValueasBool (AI|GetBlackboard (Variables|Default|GetMyAIController)) (Utilities|Name|MakeLiteralName "bAlreadyMoved") _success)
          (AI|BehaviorTree|FinishExecute _success))
        (:CastFailed
          (AI|BehaviorTree|FinishExecute false :!label _label))))
    (:CastFailed
      (goto _label))))