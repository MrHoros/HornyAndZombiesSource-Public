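; Behavior tree task that lets a zombie AI skip its move phase in the game's phase-based turn flow.
; It sets the controller's blackboard bAlreadyMoved flag to true, then calls NextPhase on the BP_GM game mode.
; The task finishes successfully when the game mode cast works and fails when it does not.
; A failed pawn or controller cast stops execution without finishing the task.
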(event EventReceiveExecuteAI
  (params (OwnerController :type AI%20Controller%20Object%20Reference) (ControlledPawn :type Pawn%20Object%20Reference))
  (bind _asbp_character_base (Utilities|Casting|CastToBP_CharacterBase ControlledPawn))
  (Variables|Default|SetMyCharacter _asbp_character_base)
  (bind _asbp_zombie_aicontroller (Utilities|Casting|CastToBP_ZombieAIController OwnerController))
  (AI|Components|Blackboard|SetValueasBool (AI|GetBlackboard _asbp_zombie_aicontroller) (Utilities|Name|MakeLiteralName "bAlreadyMoved") true)
  (bind _asbp_gm (Utilities|Casting|CastToBP_GM (Game|GetGameMode))
    (:then
      (Class|SmthTacticalGameModeBase|NextPhase _asbp_gm)
      (AI|BehaviorTree|FinishExecute true))
    (:CastFailed
      (AI|BehaviorTree|FinishExecute false))))