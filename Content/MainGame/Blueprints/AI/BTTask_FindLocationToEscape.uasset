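; Behavior tree task for zombie AI that picks a tile to flee to on the grid.
; It gathers grids reachable within the character's max stamina through the GridManager's pathfinder, then asks the GridManager for the one furthest from the human team's characters.
; That grid's center is written to the MoveLocation blackboard key, and the task fails if casts or the search come up empty.
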(event EventReceiveExecuteAI
  (params (OwnerController :type AI%20Controller%20Object%20Reference) (ControlledPawn :type Pawn%20Object%20Reference))
  (bind _asbp_zombie_aicontroller (Utilities|Casting|CastToBP_ZombieAIController OwnerController)
    (:then
      (Variables|Default|SetAIController _asbp_zombie_aicontroller)
      (bind _asbp_character_base (Utilities|Casting|CastToBP_CharacterBase ControlledPawn)
        (:then
          (Variables|Default|SetMyCharacter _asbp_character_base)
          (bind _asbp_gm (Utilities|Casting|CastToBP_GM (Game|GetGameMode))
            (:then
              (bind _output_get (Variables|Default|SetMyGamemode _asbp_gm))
              (Variables|Default|SetGrid%20Manager (Default|GetGridManager _output_get))
              (bind _result (Class|GridUtilities|GetReachableGrids (Variables|Default|GetMyCharacter) (Math|Conversions|ToFloat(Integer) (Class|STCharacterBase|GetMaxStamina (Variables|Default|GetMyCharacter))) (Class|GridManager|GetPathFinder (Variables|Default|GetGrid%20Manager))))
              (bind _furthestgrid (Default|GetFurthestGridfromTeamCharacters (Variables|Default|GetGrid%20Manager) (Default|GetHumanTeamIndex (Variables|Default|GetMyGamemode)) _result))
              (Utilities|IsValid _furthestgrid
                (:Is%20Valid
                  (AI|Components|Blackboard|SetValueasVector (AI|GetBlackboard (Variables|Default|GetAIController)) (Utilities|Name|MakeLiteralName "MoveLocation") (Class|Grid|GetCenter _furthestgrid))
                  (AI|BehaviorTree|FinishExecute true))
                (:Is%20Not%20Valid
                  (AI|BehaviorTree|FinishExecute false))))
            (:CastFailed
              (AI|BehaviorTree|FinishExecute false :!label _label))))
        (:CastFailed
          (goto _label))))
    (:CastFailed
      (goto _label))))