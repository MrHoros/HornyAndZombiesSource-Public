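; AI controller for zombie units that runs the BT_ZombieAI behavior tree.
; On BeginPlay it caches the BP_GM game mode and that mode's grid manager.
; Start launches the tree on demand and records whether it is running, and RestartBlackboardValues clears a configurable list of blackboard keys.
; GetAllAliveHumans returns the remaining characters on the human team from the game mode.
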(event EventBeginPlay
  (bind _asbp_gm (Utilities|Casting|CastToBP_GM (Game|GetGameMode)))
  (bind _output_get (Variables|Default|SetMyGamemode _asbp_gm))
  (Variables|Default|SetMyGridManager (Default|GetGridManager _output_get)))

(fn ConstructionScript)

(fn Start
  (bind _returnvalue (AI|RunBehaviorTree "/Game/MainGame/Blueprints/AI/BT_ZombieAI.BT_ZombieAI"))
  (Variables|Default|SetIsRunning _returnvalue)
  (return _returnvalue))

(fn RestartBlackboardValues
  (for _array_element (Variables|Default|GetKeysToReset)
    (AI|Components|Blackboard|ClearValue (AI|GetBlackboard self) _array_element)))

(fn GetAllAliveHumans
  (bind _mygamemode (Variables|Default|GetMyGamemode))
  (return (Default|GetRemainingCharactersOfTeamIndex _mygamemode (Default|GetHumanTeamIndex _mygamemode))))