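; Behavior tree decorator that checks whether the AI-controlled character can attack the nearest human.
; It casts the pawn to BP_CharacterBase, reads the ClosestHuman object from the blackboard, and returns that character's CanAttackCharacter result.
; The check fails if the pawn or target is invalid or not a BP_CharacterBase.
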(fn PerformConditionCheckAI
  (params (OwnerController :type AI%20Controller%20Object%20Reference) (ControlledPawn :type Pawn%20Object%20Reference))
  (bind _returnvalue (AI|GetBlackboard OwnerController))
  (bind _returnvalue_2 (Utilities|Name|MakeLiteralName "ClosestHuman"))
  (bind _returnvalue_3 (AI|Components|Blackboard|GetValueasObject _returnvalue _returnvalue_2))
  (bind _asbp_character_base (Utilities|Casting|CastToBP_CharacterBase ControlledPawn)
    (:then
      (LocalVariables|SetMyCharacter _asbp_character_base)
      (Utilities|IsValid _returnvalue_3
        (:Is%20Valid
          (bind _asbp_character_base_2 (Utilities|Casting|CastToBP_CharacterBase _returnvalue_3)
            (:then
              (return (Default|CanAttackCharacter (LocalVariables|GetMyCharacter) _asbp_character_base_2)))
            (:CastFailed
              _)))
        (:Is%20Not%20Valid
          _))
      (return false))
    (:CastFailed
      (return false))))