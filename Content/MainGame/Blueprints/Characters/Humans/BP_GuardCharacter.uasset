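; Guard character for a grid-based game, a child Blueprint that adds an area attack ability and guard-specific animation hookup.
; StartAbility plays an animation, then scans every grid within attack range and applies ability damage to each attackable character that passes a hit roll.
; It caches its BP_guard_animation instance on BeginPlay and copies the run, ability, death, damage and attack variables into it as floats.
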(event EventBeginPlay
  (|CallParentFunction)
  (bind _asbp_guard_animation (Utilities|Casting|CastToBP_guard_animation (Components|SkeletalMesh|GetAnimInstance (Variables|Character|GetMesh))))
  (Variables|Animation|SetMyAnimInstance _asbp_guard_animation))

(fn ConstructionScript
  (|CallParentFunction))

(fn UpdateAnimVariables
  (Utilities|FlowControl|Sequence
    (:then_0
      (Variables|/Game/MainGame/Mannequin/Animations/Humans/BP_guard_animation.BP_guard_animation_C|Setrun_0 (Variables|Animation|GetMyAnimInstance) (Math|Conversions|ToFloat(Integer) (Variables|Default|GetRunAnimVariable))))
    (:then_1
      (Variables|/Game/MainGame/Mannequin/Animations/Humans/BP_guard_animation.BP_guard_animation_C|Setability_0 (Variables|Animation|GetMyAnimInstance) (Math|Conversions|ToFloat(Integer) (Variables|Default|GetAbilityAnimVariable))))
    (:then_2
      (Variables|/Game/MainGame/Mannequin/Animations/Humans/BP_guard_animation.BP_guard_animation_C|Setdeath_0 (Variables|Animation|GetMyAnimInstance) (Math|Conversions|ToFloat(Integer) (Variables|Default|GetDeathAnimVariable))))
    (:then_3
      (Variables|/Game/MainGame/Mannequin/Animations/Humans/BP_guard_animation.BP_guard_animation_C|Setdamage_0 (Variables|Animation|GetMyAnimInstance) (Math|Conversions|ToFloat(Integer) (Variables|Default|GetDamagedAnimVariable))))
    (:then_4
      (Variables|/Game/MainGame/Mannequin/Animations/Humans/BP_guard_animation.BP_guard_animation_C|Setattack_0 (Variables|Animation|GetMyAnimInstance) (Math|Conversions|ToFloat(Integer) (Variables|Default|GetAttackAnimVariable))))))

(fn StartAbility
  (|CallParentFunction)
  (CallFunction|PlayAnim "NewEnumerator0")
  (bind _grids (Default|GetGridsbyRangeFloat (Variables|Default|GetMyGridManager) (Transformation|GetActorLocation) (Class|STCharacterBase|GetAttackRange)))
  (for _array_element _grids
    (Utilities|IsValid (Default|GetCharacterOverGrid (Variables|Default|GetMyGamemode) _array_element (Utilities|Array|MakeArray self))
      (:Is%20Valid
        (if (CallFunction|CanAttackCharacter (Default|GetCharacterOverGrid (Variables|Default|GetMyGamemode) _array_element (Utilities|Array|MakeArray self)))
          (bind _hit (CallFunction|RollHittoCharacter (Default|GetCharacterOverGrid (Variables|Default|GetMyGamemode) _array_element (Utilities|Array|MakeArray self))))
          (if _hit
            (Game|Damage|ApplyDamage (Default|GetCharacterOverGrid (Variables|Default|GetMyGamemode) _array_element (Utilities|Array|MakeArray self)) (Variables|Default|GetAbilityDamage) (Variables|Default|GetMyPlayerController) self)))))))

(fn OnAbilityAnimEnd
  (CallFunction|PlayAnim "NewEnumerator6")
  (|CallParentFunction))