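; Base character for turn-based grid tactics units, covering grid movement, attacks, abilities, stats display and death.
; On the first Move phase it caches manager references, binds damage and stamina events, and fills camera-facing world widgets.
; Attacks check team and range, turn both units face-to-face, then roll to hit on the animation's hit callback before reporting to BP_GM.
; PlayAnim sets state variables that child classes apply through UpdateAnimVariables, while abilities spend mod points to switch attack mode.
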(event OnArrivalGoal(GridNavigation)
  (params (Component :type Grid%20Navigation%20Component%20Object%20Reference))
  (Default|OnArrivalGoal (Variables|Default|GetMyGamemode) Component)
  (Default|OnArrivalGoal (Variables|Default|GetMyPlayerController)))

(event Custom|OnTakeAnyDamage_Event_0
  (params (DamagedActor :type Actor%20Object%20Reference) (Damage :type Float%20%28single-precision%29) (DamageType :type Damage%20Type%20Object%20Reference) (InstigatedBy :type Controller%20Object%20Reference) (DamageCauser :type Actor%20Object%20Reference))
  (bind _health (Variables|Default|GetHealth))
  ;[1 1 1] Update health displayer
  (if (== DamagedActor self)
    (Rendering|Components|TextRender|SetText (Variables|/Game/MainGame/UI/Widgets/CharacterInfo/WidgetCharacterWorldGui.WidgetCharacterWorldGui_C|GetCharacterHealth (Variables|Default|GetMyWorldInfoGui)) (Utilities|Text|ToText(Float) (Class|HealthComponent|GetHealth (Variables|Default|GetHealth)) "HalfToEven"))
    ;[1 1 1] Update health bar
    (bind _aswidget_healthbar (Utilities|Casting|CastToWidget_Healthbar (UserInterface|GetWidget (Variables|Default|GetHealthBar))))
    (Progress|SetPercent (Variables|/Game/MainGame/UI/Widgets/Widget_Healthbar.Widget_Healthbar_C|GetProgressBar_13 _aswidget_healthbar) (/ (Class|HealthComponent|GetHealth _health) (Class|HealthComponent|GetMaxHealth _health)))
    ;[1 1 1] Update game progress bar
    (Default|UpdateGameProgressBar (Variables|Default|GetMyGamemode))
    ;[1 1 1] Handle damage
    (Components|Activation|Activate (Variables|Default|GetHitVfx) true)
    (if (<= (Class|HealthComponent|GetHealth (Variables|Default|GetHealth)) 0.0)
      (Anim|PlayAnim "NewEnumerator2")
      (Audio|PlaySoundatLocation (Variables|Sound|GetDeathSound) (Transformation|GetActorLocation) "0, 0, 0" 1.0 1.0 0.0 0 0 0)
      (Utilities|FlowControl|Delay 4.5)
      (Actor|DestroyActor)
      (else
        (Anim|PlayAnim "NewEnumerator3")))))

(event Custom|LookAtRotation
  (params (Look%20at :type Rotator))
  ;[1 1 1] LookAtRotation gate
  (Utilities|FlowControl|Gate true) ; enters at Open
)

(event Custom|Dis_OnPhaseChanged_Event_0
  (params (OldPhase :type EPhase%20Enum :default "PE_None"))
  (if (Utilities|Enum|Equal(Enum) (Class|SmthTacticalGameModeBase|GetCurrentPhase (Variables|Default|GetMyGamemode)) "PE_Move")
    (Utilities|FlowControl|DoOnce false
      (:Completed
        (CallFunction|Setup)
        (Utilities|FlowControl|Sequence
          (:then_0
            ;[1 1 1] Update health displayer
            (EventDispatchers|AssignOnTakeAnyDamage (delegate Custom|OnTakeAnyDamage_Event_0)))
          (:then_1
            ;[1 1 1] Update stamina on changed
            (EventDispatchers|AssignOnStaminaChanged (delegate Custom|OnStaminaChanged_Event))))))))

(event Custom|OnStaminaChanged_Event
  (params (NewStamina :type Integer))
  ;[1 1 1] Update stamina on changed
  (bind _aswidget_character_world_gui (Utilities|Casting|CastToWidgetCharacterWorldGui (UserInterface|GetWidget (Variables|Default|GetWorldInfoGui))))
  (Rendering|Components|TextRender|SetText (Variables|/Game/MainGame/UI/Widgets/CharacterInfo/WidgetCharacterWorldGui.WidgetCharacterWorldGui_C|GetCharacterStamina _aswidget_character_world_gui) (Utilities|Text|ToText(Integer) NewStamina)))

(event EventBeginPlay
  (bind _asbp_gm (Utilities|Casting|CastToBP_GM (Game|GetGameMode)))
  (bind _output_get (Variables|Default|SetMyGamemode _asbp_gm))
  (EventDispatchers|AssignDisonPhaseChanged _output_get (delegate Custom|Dis_OnPhaseChanged_Event_0)))

(event EventTick
  (params (DeltaSeconds :type Float%20%28single-precision%29))
  (bind _returnvalue (Game|GetPlayerCameraManager 0))
  (bind _returnvalue_2 (Transformation|GetActorRotation _returnvalue))
  (bind _pitch (Math|Rotator|BreakRotator _returnvalue_2))
  (bind _returnvalue_3 (+ _pitch 1.8e+02))
  (bind _returnvalue_4 (Math|Rotator|MakeRotator 1.8e+02 _returnvalue_3 0.0))
  ;[1 1 1] Face stats and healthbar to the camera
  (Variables|Default|SetDelta%20Seconds DeltaSeconds)
  (Transformation|SetWorldRotation (Variables|Default|GetWorldInfoGui) _returnvalue_4 false false)
  (Transformation|SetWorldRotation (Variables|Default|GetHealthBar) _returnvalue_4 false false)
  ;[1 1 1] LookAtRotation gate
  (Utilities|FlowControl|Gate true :!label _label
    (:Exit
      (Transformation|SetActorRotation (Math|Interpolation|RInterpTo (Transformation|GetActorRotation) (stale Custom|LookAtRotation Look%20at) (Variables|Default|GetDelta%20Seconds) 1e+01))
      (if (Math|Rotator|Equal(Rotator) (stale Custom|LookAtRotation Look%20at) (Transformation|GetActorRotation) 1.0)
        (goto _label Close)))))

(fn ConstructionScript
  (Pawn|Components|CharacterMovement|SetMovementMode (Variables|Character|GetCharacterMovement) "MOVE_Flying" 0))

(fn Moveto
  (params (DestGrid :type Grid%20Object%20Reference) (PathFinder :type Grid%20Path%20Finder%20Object%20Reference))
  (bind _returnvalue (Class|GridNavigationComponent|RequestMove (Variables|Components|GetGridNavigation) DestGrid PathFinder))
  (return _returnvalue))

(fn GetSuggestVelocity
  (params (From :type Grid%20Object%20Reference) (To :type Grid%20Object%20Reference))
  (bind (_tossvelocity _returnvalue) (Class|GameplayStatics|BlueprintSuggestProjectileVelocity (Transformation|GetActorLocation) (Class|Grid|GetCenter To) 2e+03 0.0 "DoNotTrace" (Variables|/Script/Engine.CapsuleComponent|GetCapsuleRadius (Variables|Default|GetCapsuleComponent)) true false))
  (return _returnvalue _tossvelocity))

(fn NotifyJumpEnd
  (Default|CallJumpEndEvent self))

(fn UpdateStatDisplayer
  (bind _aswidget_character_world_gui (Utilities|Casting|CastToWidgetCharacterWorldGui (UserInterface|GetWidget (Variables|Default|GetWorldInfoGui))))
  (LocalVariables|SetStatDisplayerWidget _aswidget_character_world_gui)
  (Utilities|FlowControl|Sequence
    (:then_0
      ;[1 1 1] Damage
      (Rendering|Components|TextRender|SetText (Variables|/Game/MainGame/UI/Widgets/CharacterInfo/WidgetCharacterWorldGui.WidgetCharacterWorldGui_C|GetCharacterDamage (LocalVariables|GetStatDisplayerWidget)) (Utilities|Text|ToText(Integer) (Class|STCharacterBase|GetDamage))))
    (:then_1
      ;[1 1 1] Health
      (Rendering|Components|TextRender|SetText (Variables|/Game/MainGame/UI/Widgets/CharacterInfo/WidgetCharacterWorldGui.WidgetCharacterWorldGui_C|GetCharacterHealth (LocalVariables|GetStatDisplayerWidget)) (Utilities|Text|ToText(Float) (Class|HealthComponent|GetHealth (Variables|Default|GetHealth)) "HalfToEven")))
    (:then_2
      ;[1 1 1] MaxStamina
      (Rendering|Components|TextRender|SetText (Variables|/Game/MainGame/UI/Widgets/CharacterInfo/WidgetCharacterWorldGui.WidgetCharacterWorldGui_C|GetCharacterStamina (LocalVariables|GetStatDisplayerWidget)) (Utilities|Text|ToText(Integer) (Class|STCharacterBase|GetMaxStamina))))
    (:then_3
      ;[1 1 1] Team name
      (Rendering|Components|TextRender|SetText (Variables|/Game/MainGame/UI/Widgets/CharacterInfo/WidgetCharacterWorldGui.WidgetCharacterWorldGui_C|GetCharacterTeam (LocalVariables|GetStatDisplayerWidget)) (Utilities|Text|ToText(String) (Class|STCharacterBase|GetTeamName))))
    (:then_4
      ;[1 1 1] Character name
      (Rendering|Components|TextRender|SetText (Variables|/Game/MainGame/UI/Widgets/CharacterInfo/WidgetCharacterWorldGui.WidgetCharacterWorldGui_C|GetCharacterName (LocalVariables|GetStatDisplayerWidget)) (Utilities|Text|ToText(String) (Class|STCharacterBase|GetUnitName))))
    (:then_5
      ;[1 1 1] Attack range
      (Rendering|Components|TextRender|SetText (Variables|/Game/MainGame/UI/Widgets/CharacterInfo/WidgetCharacterWorldGui.WidgetCharacterWorldGui_C|GetCharacterAttackRange (LocalVariables|GetStatDisplayerWidget)) (Utilities|Text|ToText(Float) (Class|STCharacterBase|GetAttackRange) "HalfToEven")))
    (:then_6
      ;[1 1 1] Ach
      (Rendering|Components|TextRender|SetText (Variables|/Game/MainGame/UI/Widgets/CharacterInfo/WidgetCharacterWorldGui.WidgetCharacterWorldGui_C|GetCharacterAttackBoost (LocalVariables|GetStatDisplayerWidget)) (Utilities|Text|FormatText "+{Integer}%" (Class|STCharacterBase|GetAttackChanceBoost))))
    (:then_7
      ;[1 1 1] Dch
      (Rendering|Components|TextRender|SetText (Variables|/Game/MainGame/UI/Widgets/CharacterInfo/WidgetCharacterWorldGui.WidgetCharacterWorldGui_C|GetCharacterDefenseBoost (LocalVariables|GetStatDisplayerWidget)) (Utilities|Text|FormatText "+{Integer}%" (Class|STCharacterBase|GetDefenseChanceBoost))))
    (:then_8
      ;[1 0.9796 0.5782] Colors
      (Appearance|SetColorandOpacity (Variables|/Game/MainGame/UI/Widgets/CharacterInfo/WidgetCharacterWorldGui.WidgetCharacterWorldGui_C|GetCharacterTeam (LocalVariables|GetStatDisplayerWidget)) (Utilities|Struct|MakeSlateColor (Math|Conversions|ToLinearColor(Color) (Class|STCharacterBase|GetTeamColor)) (.ColorUseRule (Utilities|Struct|BreakSlateColor (Variables|/Script/UMG.TextBlock|GetColorAndOpacity (Variables|/Game/MainGame/UI/Widgets/CharacterInfo/WidgetCharacterWorldGui.WidgetCharacterWorldGui_C|GetCharacterTeam (LocalVariables|GetStatDisplayerWidget)))))) :!class /Script/UMG.TextBlock)
      (Appearance|SetColorandOpacity (Variables|/Game/MainGame/UI/Widgets/CharacterInfo/WidgetCharacterWorldGui.WidgetCharacterWorldGui_C|GetCharacterName (LocalVariables|GetStatDisplayerWidget)) (Utilities|Struct|MakeSlateColor (Math|Conversions|ToLinearColor(Color) (Class|STCharacterBase|GetTeamColor)) (.ColorUseRule (Utilities|Struct|BreakSlateColor (Variables|/Script/UMG.TextBlock|GetColorAndOpacity (Variables|/Game/MainGame/UI/Widgets/CharacterInfo/WidgetCharacterWorldGui.WidgetCharacterWorldGui_C|GetCharacterTeam (LocalVariables|GetStatDisplayerWidget)))))) :!class /Script/UMG.TextBlock))))

(fn GetWorldGui
  (bind _aswidget_character_world_gui (Utilities|Casting|CastToWidgetCharacterWorldGui (UserInterface|GetWidget (Variables|Default|GetWorldInfoGui))))
  (return _aswidget_character_world_gui))

(fn GetMyHealthComponent
  (return (Variables|Default|GetHealth)))

(fn PlayAnim
  (params (Anim :type CharacterAnims%20Enum :default "NewEnumerator0"))
  (if (Utilities|Enum|NotEqual(Enum) Anim "NewEnumerator6")
    (Anim|PlayAnim "NewEnumerator6"))
  (switch Utilities|FlowControl|Switch|SwitchonCharacterAnims Anim
    (:NewEnumerator0
      (Variables|Animation|SetAbilityAnimVariable 1))
    (:NewEnumerator1
      (Variables|Animation|SetAttackAnimVariable 1))
    (:NewEnumerator2
      (Variables|Animation|SetDeathAnimVariable 1))
    (:NewEnumerator3
      (Variables|Animation|SetDamagedAnimVariable 1))
    (:NewEnumerator4
      (Variables|Animation|SetBirthAnimVariable 1))
    (:NewEnumerator5
      (Variables|Animation|SetRunAnimVariable 1))
    (:NewEnumerator6
      (Variables|Animation|SetRunAnimVariable 0)
      (Variables|Animation|SetAbilityAnimVariable 0)
      (Variables|Animation|SetDeathAnimVariable 0)
      (Variables|Animation|SetAttackAnimVariable 0)
      (Variables|Animation|SetBirthAnimVariable 0)
      (Variables|Animation|SetDamagedAnimVariable 0)))
  (Anim|UpdateAnimVariables))

(fn UpdateAnimVariables
  ;[1 1 1] Define in animatable child class
)

(fn IsActorinAttackRange
  (params (Actor :type Actor%20Object%20Reference))
  (LocalVariables|SetTargetActor Actor)
  (bind _returnvalue (Class|GridManager|GetGridbyPosition (Variables|Default|GetMyGridManager) (Transformation|GetActorLocation)))
  (LocalVariables|SetStart (Class|Grid|GetCenter _returnvalue))
  (bind _returnvalue_2 (Class|GridManager|GetGridbyPosition (Variables|Default|GetMyGridManager) (Transformation|GetActorLocation (LocalVariables|GetTargetActor))))
  (LocalVariables|SetTarget (Class|Grid|GetCenter _returnvalue_2))
  (return (<= (Math|Vector|Distance(Vector) (LocalVariables|GetStart) (LocalVariables|GetTarget)) (* (Class|STCharacterBase|GetAttackRange) 1e+02))))

(fn AttackCharacter
  (params (Target :type BP%20Character%20Base%20Object%20Reference))
  (bind _output_get (Variables|Default|SetAttackTarget Target))
  (if (CallFunction|CanAttackCharacter _output_get)
    (CallFunction|RotateFacetoFace (Variables|Default|GetAttackTarget))
    (Anim|PlayAnim "NewEnumerator1")
    (return true)
    (else
      (return false))))

(fn IsGridCharacterinSight
  (params (Grid :type Grid%20Object%20Reference))
  (bind _output_get (LocalVariables|SetMyGrid Grid))
  (bind _output_get_2 (LocalVariables|SetCharacterOverGrid (Default|GetCharacterOverGrid (Variables|Default|GetMyGamemode) _output_get (Utilities|Array|MakeArray self))))
  (Utilities|IsValid _output_get_2
    (:Is%20Valid
      (if (CallFunction|ShouldIgnoreGivenCharacter (LocalVariables|GetCharacterOverGrid))
        (LocalVariables|SetActorsToIgnore (Utilities|Array|MakeArray self (LocalVariables|GetCharacterOverGrid)))
        (else
          (LocalVariables|SetActorsToIgnore (Utilities|Array|MakeArray 0) :!label _label))))
    (:Is%20Not%20Valid
      (goto _label)))
  (bind _returnvalue (Collision|LineTraceByChannel (+ (Class|Grid|GetCenter (LocalVariables|GetMyGrid)) "0, 0,80.000000") (Transformation|GetActorLocation) "TraceTypeQuery1" true (LocalVariables|GetActorsToIgnore) "None"))
  (return (not _returnvalue)))

(fn ShouldIgnoreGivenCharacter
  (params (Character%20to%20check :type ST%20Character%20Base%20Object%20Reference))
  (return (!= (Class|STCharacterBase|GetTeamIndex Character%20to%20check) (Class|STCharacterBase|GetTeamIndex))))

(fn GetAttackMode
  (return (Variables|Default|GetAttackMode)))

(fn StartAbility
  (bind _myplayercontroller (Variables|Default|GetMyPlayerController))
  (if (>= (Class|STCharacterBase|GetModPoints) (CallFunction|GetAbilityCost))
    (if (Variables|/Game/MainGame/Blueprints/Core/BP_STPlayerController.BP_STPlayerController_C|GetAttackDebounce _myplayercontroller)
      _
      (else
        (Variables|/Game/MainGame/Blueprints/Core/BP_STPlayerController.BP_STPlayerController_C|SetAttackDebounce _myplayercontroller true)))
    (Class|STCharacterBase|ChangeModPoints (* (CallFunction|GetAbilityCost) -1))
    (CallFunction|SetAttackMode "NewEnumerator1")
    (Default|SetSquareAttackableMaterial (Variables|Default|GetMyDecalPainter) "/Game/MainGame/Materials/M_SquareGrid_Ability.M_SquareGrid_Ability")))

(fn OnAbilityAnimEnd
  (CallFunction|SetAttackMode "NewEnumerator0")
  (Default|AbilityEndEvent (Variables|Default|GetMyGamemode))
  (return))

(fn OnAttackAnimHit
  (bind _attacktarget (Variables|Default|GetAttackTarget))
  (Audio|PlaySoundatLocation (Variables|Sound|GetAttackSound) (Transformation|GetActorLocation) "0, 0, 0" 1.0 1.0 0.0 0 0 0)
  (Utilities|IsValid _attacktarget
    (:Is%20Valid
      (bind _hit (CallFunction|RollHittoCharacter _attacktarget))
      (if _hit
        (Game|Damage|ApplyDamage (Variables|Default|GetAttackTarget) (Math|Conversions|ToFloat(Integer) (Class|STCharacterBase|GetDamage)) (Game|GetPlayerController 0) self "/Script/Engine.DamageType"))
      (Default|AttackEndEvent (Variables|Default|GetMyGamemode))
      (return))))

(fn OnAttackAnimEnd
  (Anim|PlayAnim "NewEnumerator6")
  (return))

(fn OnDamagedAnimEnd
  (Anim|PlayAnim "NewEnumerator6")
  (return))

(fn Setup
  (bind _asbp_stplayer_controller (Utilities|Casting|CastToBP_STPlayerController (Game|GetPlayerController 0)))
  (Variables|Default|SetMyPlayerController _asbp_stplayer_controller)
  (Variables|Default|SetMyGridManager (Default|GetGridManager (Variables|Default|GetMyGamemode)))
  (bind _aswidget_character_world_gui (Utilities|Casting|CastToWidgetCharacterWorldGui (UserInterface|GetWidget (Variables|Default|GetWorldInfoGui))))
  (Variables|Default|SetMyWorldInfoGui _aswidget_character_world_gui)
  (Class|STCharacterBase|AssignBaseDefenseChance)
  (UI|UpdateStatDisplayer)
  (bind _asmy_grid_decal_painter (Utilities|Casting|CastToMyGridDecalPainter (Class|GridManager|GetGridPainter (Variables|Default|GetMyGridManager))))
  (Variables|Default|SetMyDecalPainter _asmy_grid_decal_painter)
  (CallFunction|UpdateAbilityInfo))

(fn SetAttackMode
  (params (Mode :type AttackModeEnum%20Enum :default "NewEnumerator0"))
  (Variables|Default|SetAttackMode Mode)
  (return))

(fn GetAbilityCost
  (return (Variables|Default|GetAbilityCost)))

(fn OnAbilityRightClickedActor
  (params (ActorClicked :type Actor%20Object%20Reference))
  (return))

(fn RotateFacetoFace
  (params (OtherCharacter :type BP%20Character%20Base%20Object%20Reference))
  (LocalVariables|SetRotateTarget OtherCharacter)
  (CallFunction|LookatRotation (Math|Rotator|FindLookatRotation (Transformation|GetActorLocation self) (Transformation|GetActorLocation (LocalVariables|GetRotateTarget))))
  (CallFunction|LookatRotation (LocalVariables|GetRotateTarget) (Math|Rotator|FindLookatRotation (Transformation|GetActorLocation (LocalVariables|GetRotateTarget)) (Transformation|GetActorLocation self))))

(fn CanAttackCharacter
  (params (TargetCharacter :type ST%20Character%20Base%20Object%20Reference))
  (bind _output_get (LocalVariables|SetMyTargetCharacter TargetCharacter))
  (return (and (!= (Class|STCharacterBase|GetTeamIndex _output_get) (Class|STCharacterBase|GetTeamIndex)) (CallFunction|IsActorinAttackRange (LocalVariables|GetMyTargetCharacter)))))

(fn RollHittoCharacter
  (params (Defender :type BP%20Character%20Base%20Object%20Reference))
  (Utilities|IsValid Defender
    (:Is%20Valid
      (if (<= (Math|Random|RandomInteger 100) (Class|STCharacterBase|GetChancetoAttackCharacter Defender))
        (Development|PrintString "HIT!")
        (Audio|PlaySoundatLocation (Variables|Sound|GetAttackSoundHit) (Transformation|GetActorLocation) "0, 0, 0" 1.0 1.0 0.0 0 0 0)
        (return true)
        (else
          (Development|PrintString "MISS!")
          (Audio|PlaySoundatLocation (Variables|Sound|GetAttackSoundMiss) (Transformation|GetActorLocation) "0, 0, 0" 1.0 1.0 0.0 0 0 0)
          (return false))))))

(fn OnAbilityAnimHit
  (Audio|PlaySoundatLocation (Variables|Sound|GetAbilityHitSound) (Transformation|GetActorLocation) "0, 0, 0" 1.0 1.0 0.0 0 0 0)
  (return))

(fn OnIdleAnimStart
  (bind _spawnedwalksound (Variables|Default|GetSpawnedWalkSound))
  (Utilities|IsValid _spawnedwalksound
    (:Is%20Valid
      (Audio|Components|Audio|Stop _spawnedwalksound)
      (return))))

(fn OnWalkAnimStart
  (Utilities|IsValid (Variables|Default|GetSpawnedWalkSound)
    (:Is%20Valid
      (Audio|Components|Audio|Play (Variables|Default|GetSpawnedWalkSound) 0.0))
    (:Is%20Not%20Valid
      (bind _returnvalue (Audio|SpawnSoundAttached (Variables|Sound|GetWalkSound) (Variables|Default|GetCapsuleComponent) "None" "0, 0, 0" "0, 0, 0" "KeepRelativeOffset" true 1.0 1.0 0.0 0 0 false))
      (Variables|Default|SetSpawnedWalkSound _returnvalue)))
  (return))

(fn OnDamagedAnimStart
  (Audio|PlaySoundatLocation (Variables|Sound|GetDamagedSound) (Transformation|GetActorLocation) "0, 0, 0" 1.0 1.0 0.0 0 0 0)
  (return))

(fn GetMaxCostinCurrentPhase
  (switch Utilities|FlowControl|Switch|SwitchonEPhase (Class|SmthTacticalGameModeBase|GetCurrentPhase (Variables|Default|GetMyGamemode))
    (:PE_Move
      (return (+ (Math|Conversions|ToFloat(Integer) (Class|STCharacterBase|GetStamina)) (Class|STCharacterBase|GetAttackRange))))
    (:PE_Attack
      (return (Class|STCharacterBase|GetAttackRange)))))

(fn HideStatDsiplayer
  (bind _newparam (UI|GetWorldGui))
  (Default|SetAllCanvasVisibleState _newparam "Hidden"))

(fn IsAIControlled
  (return (== (Utilities|GetClass (AI|GetAIController self)) (Default|GetZombieAIClass (Variables|Default|GetMyGamemode)))))

(fn RestartAttackMode
  (Variables|Default|SetAttackMode "NewEnumerator0"))

(fn GetAIMovementMode
  (return (Variables|Default|GetAIMovementMode)))

(fn UpdateAbilityInfo
  (bind _aswidget_character_world_gui (Utilities|Casting|CastToWidgetCharacterWorldGui (UserInterface|GetWidget (Variables|Default|GetWorldInfoGui))))
  (Utilities|FlowControl|Sequence
    (:then_0
      (Default|ChangeAbilityIcon _aswidget_character_world_gui (Variables|Default|GetAbilityIcon)))
    (:then_1
      (Default|ChangeAbilityName _aswidget_character_world_gui (Variables|Default|GetAbilityName)))))

(fn GetMyHealthbarWidget)

(fn GetGridManager
  (return (Default|GetGridManager (Variables|Default|GetMyGamemode))))