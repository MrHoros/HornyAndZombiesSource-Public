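; Behavior Tree task that picks where an AI-controlled zombie moves on the grid to chase its closest human.
; It gets the grids reachable within the character's max stamina, then keeps the one nearest the ClosestHuman blackboard target, without resetting the stored closest distance between runs.
; It writes that grid's center to MoveLocation and succeeds, failing if the character already stands there or a cast fails.
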(event EventReceiveExecuteAI
  (params (OwnerController :type AI%20Controller%20Object%20Reference) (ControlledPawn :type Pawn%20Object%20Reference))
  (bind _asbp_zombie_aicontroller (Utilities|Casting|CastToBP_ZombieAIController OwnerController)
    (:then
      (Variables|Default|SetAIController _asbp_zombie_aicontroller)
      (bind _asbp_character_base (Utilities|Casting|CastToBP_CharacterBase ControlledPawn)
        (:then
          (Variables|Default|SetMyCharacter _asbp_character_base)
          (bind _asbp_gm (Utilities|Casting|CastToBP_GM (Game|GetGameMode))
            (:then
              (bind _output_get (Variables|Default|SetMyGamemode _asbp_gm))
              (Variables|Default|SetGrid%20Manager (Default|GetGridManager _output_get))
              (bind _asbp_character_base_2 (Utilities|Casting|CastToBP_CharacterBase (AI|Components|Blackboard|GetValueasObject (AI|GetBlackboard (Variables|Default|GetAIController)) (Utilities|Name|MakeLiteralName "ClosestHuman")))
                (:then
                  (Variables|Default|SetTargetHuman _asbp_character_base_2)
                  (bind _result (Class|GridUtilities|GetReachableGrids (Variables|Default|GetMyCharacter) (Math|Conversions|ToFloat(Integer) (Class|STCharacterBase|GetMaxStamina (Variables|Default|GetMyCharacter))) (Class|GridManager|GetPathFinder (Variables|Default|GetGrid%20Manager))))
                  (for _array_element _result
                    (Math|Float|CompareFloat (Math|Vector|Distance(Vector) (Class|Grid|GetCenter _array_element) (Transformation|GetActorLocation (Variables|Default|GetTargetHuman))) (Variables|Default|GetClosestDistance)
                      (:<
                        (Variables|Default|SetClosestDistance (Math|Vector|Distance(Vector) (Class|Grid|GetCenter _array_element) (Transformation|GetActorLocation (Variables|Default|GetTargetHuman))))
                        (Variables|Default|SetClosestGrid _array_element))))
                  (bind _returnvalue (Class|GridManager|GetGridbyPosition (Variables|Default|GetGrid%20Manager) (Transformation|GetActorLocation (Variables|Default|GetMyCharacter))))
                  (if (not (Math|Vector|Equal(Vector) (Class|Grid|GetCenter _returnvalue) (Class|Grid|GetCenter (Variables|Default|GetClosestGrid)) 5e+01))
                    (AI|Components|Blackboard|SetValueasVector (AI|GetBlackboard (Variables|Default|GetAIController)) (Utilities|Name|MakeLiteralName "MoveLocation") (Class|Grid|GetCenter (Variables|Default|GetClosestGrid)))
                    (AI|BehaviorTree|FinishExecute true)
                    (else
                      (AI|BehaviorTree|FinishExecute false))))
                (:CastFailed
                  (AI|BehaviorTree|FinishExecute false :!label _label))))
            (:CastFailed
              (goto _label))))
        (:CastFailed
          (goto _label))))
    (:CastFailed
      (goto _label))))