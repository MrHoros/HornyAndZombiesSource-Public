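; Intern human character that adds a self-damaging targeted attack ability on top of its parent's ability hooks.
; Starting the ability boosts attack chance, and right-clicking an attackable character turns to face it and plays an animation.
; The hit damages both target and Intern, and animation end restores the default attackable decal material.
; Animation state is copied to the cached intern AnimInstance only while its ability value is not positive.
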(event OnComponentDeactivated(Health)
  (params (Component :type Actor%20Component%20Object%20Reference)))

(event EventBeginPlay
  (|CallParentFunction)
  (bind _asbp_intern_animation (Utilities|Casting|CastToBP_intern_animation (Components|SkeletalMesh|GetAnimInstance (Variables|Character|GetMesh))))
  (Variables|Animation|SetMyAnimInstance _asbp_intern_animation))

(fn ConstructionScript
  (|CallParentFunction))

(fn UpdateAnimVariables
  (if (<= (Variables|/Game/MainGame/Mannequin/Animations/Humans/BP_intern_animation.BP_intern_animation_C|Getability_0 (Variables|Animation|GetMyAnimInstance)) 0.0)
    (Utilities|FlowControl|Sequence
      (:then_0
        (Variables|/Game/MainGame/Mannequin/Animations/Humans/BP_intern_animation.BP_intern_animation_C|Setrun_0 (Variables|Animation|GetMyAnimInstance) (Math|Conversions|ToFloat(Integer) (Variables|Default|GetRunAnimVariable))))
      (:then_1
        (Variables|/Game/MainGame/Mannequin/Animations/Humans/BP_intern_animation.BP_intern_animation_C|Setability_0 (Variables|Animation|GetMyAnimInstance) (Math|Conversions|ToFloat(Integer) (Variables|Default|GetAbilityAnimVariable))))
      (:then_2
        (Variables|/Game/MainGame/Mannequin/Animations/Humans/BP_intern_animation.BP_intern_animation_C|Setdeath_0 (Variables|Animation|GetMyAnimInstance) (Math|Conversions|ToFloat(Integer) (Variables|Default|GetDeathAnimVariable))))
      (:then_3
        (Variables|/Game/MainGame/Mannequin/Animations/Humans/BP_intern_animation.BP_intern_animation_C|Setdamage_0 (Variables|Animation|GetMyAnimInstance) (Math|Conversions|ToFloat(Integer) (Variables|Default|GetDamagedAnimVariable))))
      (:then_4
        (Variables|/Game/MainGame/Mannequin/Animations/Humans/BP_intern_animation.BP_intern_animation_C|Setattack_0 (Variables|Animation|GetMyAnimInstance) (Math|Conversions|ToFloat(Integer) (Variables|Default|GetAttackAnimVariable)))))))

(fn StartAbility
  (|CallParentFunction)
  (Class|STCharacterBase|SetAttackChanceBoost 100))

(fn OnAbilityRightClickedActor
  (params (ActorClicked :type Actor%20Object%20Reference))
  (|CallParentFunction 0)
  (bind _asbp_character_base (Utilities|Casting|CastToBP_CharacterBase ActorClicked))
  (bind _output_get (Variables|Default|SetAbilityCharacterClicked _asbp_character_base))
  (if (CallFunction|CanAttackCharacter _output_get)
    (CallFunction|RotateFacetoFace (Variables|Default|GetAbilityCharacterClicked))
    (CallFunction|PlayAnim "NewEnumerator0")))

(fn OnAbilityAnimEnd
  (Default|SetDefaultAttackableMaterial (Variables|Default|GetMyDecalPainter))
  (|CallParentFunction))

(fn OnAbilityAnimHit
  (|CallParentFunction)
  (Game|Damage|ApplyDamage (Variables|Default|GetAbilityCharacterClicked) (Variables|Default|GetAbilityDamage) (Variables|Default|GetMyPlayerController) self "/Script/Engine.DamageType")
  (Game|Damage|ApplyDamage self 1e+02 (Variables|Default|GetMyPlayerController) (Variables|Default|GetAbilityCharacterClicked) "/Script/Engine.DamageType"))