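; BP_CeoCharacter is the CEO human character, whose ability is a multi-shot attack on clicked characters.
; StartAbility refills the shot count; each right-click on a character spends a shot, then faces and animates if the target is attackable.
; The hit event rolls to hit before applying damage, and animation end either allows another shot or ends the ability through the gamemode.
; UpdateAnimVariables copies state into the CEO animation instance.
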(event EventBeginPlay
  (|CallParentFunction)
  (bind _asbp_ceo_animation (Utilities|Casting|CastToBP_ceo_animation (Components|SkeletalMesh|GetAnimInstance (Variables|Character|GetMesh))))
  (Variables|Animation|SetMyAnimInstance _asbp_ceo_animation))

(fn ConstructionScript
  (|CallParentFunction))

(fn UpdateAnimVariables
  (Utilities|FlowControl|Sequence
    (:then_0
      (Variables|/Game/MainGame/Mannequin/Animations/Humans/BP_ceo_animation.BP_ceo_animation_C|Setwalk_0 (Variables|Animation|GetMyAnimInstance) (Math|Conversions|ToFloat(Integer) (Variables|Default|GetRunAnimVariable))))
    (:then_1
      (Variables|/Game/MainGame/Mannequin/Animations/Humans/BP_ceo_animation.BP_ceo_animation_C|Setability_0 (Variables|Animation|GetMyAnimInstance) (Math|Conversions|ToFloat(Integer) (Variables|Default|GetAbilityAnimVariable))))
    (:then_2
      (Variables|/Game/MainGame/Mannequin/Animations/Humans/BP_ceo_animation.BP_ceo_animation_C|Setdeath_0 (Variables|Animation|GetMyAnimInstance) (Math|Conversions|ToFloat(Integer) (Variables|Default|GetDeathAnimVariable))))
    (:then_3
      (Variables|/Game/MainGame/Mannequin/Animations/Humans/BP_ceo_animation.BP_ceo_animation_C|Setdamage_0 (Variables|Animation|GetMyAnimInstance) (Math|Conversions|ToFloat(Integer) (Variables|Default|GetDamagedAnimVariable))))
    (:then_4
      (Variables|/Game/MainGame/Mannequin/Animations/Humans/BP_ceo_animation.BP_ceo_animation_C|Setattack_0 (Variables|Animation|GetMyAnimInstance) (Math|Conversions|ToFloat(Integer) (Variables|Default|GetAttackAnimVariable))))))

(fn OnAbilityRightClickedActor
  (params (ActorClicked :type Actor%20Object%20Reference))
  (|CallParentFunction 0)
  (bind _asbp_character_base (Utilities|Casting|CastToBP_CharacterBase ActorClicked))
  (Variables|Default|SetCharacterClicked _asbp_character_base)
  (Math|Integer|CompareInt (Variables|Default|GetCurrentAbilityShots)
    (:>
      (Math|Integer|DecrementInt (Variables|Default|GetCurrentAbilityShots)
        (:%20%20
          (if (CallFunction|CanAttackCharacter (Variables|Default|GetCharacterClicked))
            (CallFunction|RotateFacetoFace (Variables|Default|GetCharacterClicked))
            (CallFunction|PlayAnim "NewEnumerator0")))))))

(fn OnAbilityAnimEnd
  (Math|Integer|CompareInt (Variables|Default|GetCurrentAbilityShots)
    (:>
      (Variables|/Game/MainGame/Blueprints/Core/BP_STPlayerController.BP_STPlayerController_C|SetAttackDebounce (Variables|Default|GetMyPlayerController) false)
      (CallFunction|PlayAnim "NewEnumerator6"))
    (:==
      (CallFunction|SetAttackMode "NewEnumerator0" :!label _label)
      (CallFunction|PlayAnim "NewEnumerator6")
      (Default|AbilityEndEvent (Variables|Default|GetMyGamemode)))
    (:<
      (goto _label))))

(fn StartAbility
  (|CallParentFunction)
  (Variables|Default|SetCurrentAbilityShots (Variables|Default|GetMaxAbilityShots)))

(fn OnAbilityAnimHit
  (|CallParentFunction)
  (bind _hit (CallFunction|RollHittoCharacter (Variables|Default|GetCharacterClicked)))
  (if _hit
    (Game|Damage|ApplyDamage (Variables|Default|GetCharacterClicked) (Variables|Default|GetAbilityDamage) (Variables|Default|GetMyPlayerController) self "/Script/Engine.DamageType")))