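; Zombie nurse enemy for a grid-based, round-driven game that summons zombie intern minions every second round end.
; SpawnMinion gathers same-height grids in range, uses downward line traces to keep unblocked ones, picks one at random, faces it and plays an animation.
; When the ability animation ends, it spawns the intern there and rebuilds the gamemode's character priority.
; UpdateAnimVariables copies animation state variables into the nurse's anim instance.
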(event Custom|Dis_OnRoundEnd_Event_0
  (bind _result (Math|Integer|IncrementInt (Variables|Default|GetPhaseCounter))
    (:%20%20
      (if (>= _result 2)
        (Variables|Default|SetPhaseCounter 0)
        (CallFunction|SpawnMinion)))))

(event EventBeginPlay
  (|CallParentFunction)
  (bind _asbp_zombie_nurse_animation (Utilities|Casting|CastToBP_zombie_nurse_animation (Components|SkeletalMesh|GetAnimInstance (Variables|Character|GetMesh))))
  (Variables|Animation|SetMyAnimInstance _asbp_zombie_nurse_animation)
  (EventDispatchers|AssignDisonRoundEnd (Variables|Default|GetMyGamemode) (delegate Custom|Dis_OnRoundEnd_Event_0)))

(fn ConstructionScript
  (|CallParentFunction))

(fn UpdateAnimVariables
  (Utilities|FlowControl|Sequence
    (:then_0
      (Variables|/Game/MainGame/Mannequin/Animations/Zombies/BP_zombie_nurse_animation.BP_zombie_nurse_animation_C|Setwalk_0 (Variables|Animation|GetMyAnimInstance) (Math|Conversions|ToFloat(Integer) (Variables|Default|GetRunAnimVariable))))
    (:then_1
      (Variables|/Game/MainGame/Mannequin/Animations/Zombies/BP_zombie_nurse_animation.BP_zombie_nurse_animation_C|Setdeath_0 (Variables|Animation|GetMyAnimInstance) (Math|Conversions|ToFloat(Integer) (Variables|Default|GetDeathAnimVariable))))
    (:then_2
      (Variables|/Game/MainGame/Mannequin/Animations/Zombies/BP_zombie_nurse_animation.BP_zombie_nurse_animation_C|Setdamage_0 (Variables|Animation|GetMyAnimInstance) (Math|Conversions|ToFloat(Integer) (Variables|Default|GetDamagedAnimVariable))))
    (:then_3
      (Variables|/Game/MainGame/Mannequin/Animations/Zombies/BP_zombie_nurse_animation.BP_zombie_nurse_animation_C|Setattack_0 (Variables|Animation|GetMyAnimInstance) (Math|Conversions|ToFloat(Integer) (Variables|Default|GetAttackAnimVariable))))
    (:then_4
      (Variables|/Game/MainGame/Mannequin/Animations/Zombies/BP_zombie_nurse_animation.BP_zombie_nurse_animation_C|Setability_0 (Variables|Animation|GetMyAnimInstance) (Math|Conversions|ToFloat(Integer) (Variables|Default|GetAbilityAnimVariable))))))

(fn SpawnMinion
  (bind _returnvalue (Class|GridManager|GetGridbyPosition (Variables|Default|GetMyGridManager) (Transformation|GetActorLocation)))
  (bind _output_get (LocalVariables|SetStartGridCenter (Class|Grid|GetCenter _returnvalue)))
  (bind _grids (Default|GetGridsbyRangeFloat (Variables|Default|GetMyGridManager) _output_get (Variables|Default|GetMinionSpawnRange)))
  (for _array_element _grids
    (bind _output_get_2 (Variables|Default|SetArray%20Element _array_element))
    (if (== (.Z (Math|Vector|BreakVector (LocalVariables|GetStartGridCenter))) (.Z (Math|Vector|BreakVector (Class|Grid|GetCenter _output_get_2))))
      (bind _returnvalue_2 (Collision|LineTraceByChannel (+ (Class|Grid|GetCenter _output_get_2) "0, 0,500.000000") (+ (Class|Grid|GetCenter _output_get_2) "0,0.000000,1.000000") "TraceTypeQuery1" false 0 "None" false))
      (if (not _returnvalue_2)
        (Utilities|Array|Add (LocalVariables|GetPossibleGrids) (Variables|Default|GetArray%20Element)))))
  (if (> (Utilities|Array|Length (LocalVariables|GetPossibleGrids)) 0)
    (Variables|Default|SetMinionSpawnLocation (Class|Grid|GetCenter (.OutItem (Utilities|Array|Random (LocalVariables|GetPossibleGrids)))))
    (CallFunction|LookatRotation (Math|Rotator|FindLookatRotation (* (Transformation|GetActorLocation self) "1.000000,1.000000,0.000000") (* (Variables|Default|GetMinionSpawnLocation) "1.000000,1.000000,0.000000")))
    (CallFunction|PlayAnim "NewEnumerator0")))

(fn OnAbilityAnimEnd
  (|CallParentFunction)
  (bind _returnvalue (Class|CharacterSpawnerComponent|SpawnCharacteratLocation (Variables|Default|GetCharacterSpawner) "/Game/MainGame/Blueprints/Characters/Zombies/BP_ZombieInternCharacter.BP_ZombieInternCharacter_C" (+ (Variables|Default|GetMinionSpawnLocation) "0, 0,82.000000")))
  (bind _asbp_character_base (Utilities|Casting|CastToBP_CharacterBase _returnvalue))
  (Default|PlayAnim _asbp_character_base "NewEnumerator4")
  (Default|RecreateMyCharactersPriority (Variables|Default|GetMyGamemode)))