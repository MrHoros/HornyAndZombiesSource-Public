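; Nurse character for turn-based grid combat whose attack action heals a character instead of damaging it.
; AttackCharacter forwards to HealCharacter, which, for targets in range, turns to face them, plays animation and sound, then adds health equal to its damage stat, capped at full.
; On its turn's Attack phase, it swaps the attackable-square decal to a healable material.
; Setup binds that phase event and caches the nurse AnimInstance fed by UpdateAnimVariables.
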(event Custom|EventConnectOnPhaseChanged
  (EventDispatchers|AssignDisonPhaseChanged (Variables|Default|GetMyGamemode) (delegate Custom|Dis_OnPhaseChanged_Event_1)))

(event Custom|Dis_OnPhaseChanged_Event_1
  (params (OldPhase :type EPhase%20Enum :default "PE_None"))
  (if (== self (Default|GetCurrentTurnCharacter (Variables|Default|GetMyGamemode)))
    (switch Utilities|FlowControl|Switch|SwitchonEPhase (Class|SmthTacticalGameModeBase|GetCurrentPhase (Variables|Default|GetMyGamemode))
      (:PE_Attack
        (Default|SetSquareAttackableMaterial (Variables|Default|GetMyDecalPainter) "/Game/MainGame/Materials/M_SquareGrid_Healable.M_SquareGrid_Healable")))))

(event EventBeginPlay
  (|CallParentFunction))

(fn ConstructionScript
  (|CallParentFunction))

(fn UpdateAnimVariables
  (Utilities|FlowControl|Sequence
    (:then_0
      (Variables|/Game/MainGame/Mannequin/Animations/Humans/BP_nurse_animation.BP_nurse_animation_C|Setrun_0 (Variables|Animation|GetMyAnimInstance) (Math|Conversions|ToFloat(Integer) (Variables|Default|GetRunAnimVariable))))
    (:then_1
      (Variables|/Game/MainGame/Mannequin/Animations/Humans/BP_nurse_animation.BP_nurse_animation_C|Setability_0 (Variables|Animation|GetMyAnimInstance) (Math|Conversions|ToFloat(Integer) (Variables|Default|GetAbilityAnimVariable))))
    (:then_2
      (Variables|/Game/MainGame/Mannequin/Animations/Humans/BP_nurse_animation.BP_nurse_animation_C|Setdeath_0 (Variables|Animation|GetMyAnimInstance) (Math|Conversions|ToFloat(Integer) (Variables|Default|GetDeathAnimVariable))))
    (:then_3
      (Variables|/Game/MainGame/Mannequin/Animations/Humans/BP_nurse_animation.BP_nurse_animation_C|Setdamage_0 (Variables|Animation|GetMyAnimInstance) (Math|Conversions|ToFloat(Integer) (Variables|Default|GetDamagedAnimVariable))))))

(fn ShouldIgnoreGivenCharacter
  (params (Character%20to%20check :type ST%20Character%20Base%20Object%20Reference))
  (return (== (Class|STCharacterBase|GetTeamIndex Character%20to%20check) (Class|STCharacterBase|GetTeamIndex))))

(fn AttackCharacter
  (params (Target :type BP%20Character%20Base%20Object%20Reference))
  (bind _success (CallFunction|HealCharacter Target))
  (return _success))

(fn HealCharacter
  (params (Character :type ST%20Character%20Base%20Object%20Reference))
  (if (== (Class|STCharacterBase|GetTeamIndex) (Class|STCharacterBase|GetTeamIndex))
    (LocalVariables|SetTeammate Character)
    (if (CallFunction|IsActorinAttackRange (LocalVariables|GetTeammate))
      (CallFunction|LookatRotation (Math|Rotator|FindLookatRotation (Transformation|GetActorLocation self) (Transformation|GetActorLocation (LocalVariables|GetTeammate))))
      (CallFunction|PlayAnim "NewEnumerator0")
      (Audio|PlaySoundatLocation (Variables|Sound|GetHealSound) (Transformation|GetActorLocation) "0, 0, 0" 1.0 1.0 0.0 0 0 0)
      (bind _asbp_character_base (Utilities|Casting|CastToBP_CharacterBase (LocalVariables|GetTeammate))
        (:then
          (LocalVariables|SetMateHealthComponent (Default|GetMyHealthComponent _asbp_character_base))
          (Math|Float|CompareFloat (Class|HealthComponent|GetMissingHealth (Default|GetMyHealthComponent _asbp_character_base)) (Math|Conversions|ToFloat(Integer) (Class|STCharacterBase|GetDamage))
            (:>
              (Class|HealthComponent|ChangeHealth (LocalVariables|GetMateHealthComponent) (Math|Conversions|ToFloat(Integer) (Class|STCharacterBase|GetDamage))))
            (:==
              (Class|HealthComponent|RestoreHealth (LocalVariables|GetMateHealthComponent) :!label _label))
            (:<
              (goto _label)))
          (return true))
        (:CastFailed
          (return false)))
      (else
        (return false)))
    (else
      (return false))))

(fn Setup
  (|CallParentFunction)
  (bind _asbp_nurse_animation (Utilities|Casting|CastToBP_nurse_animation (Components|SkeletalMesh|GetAnimInstance (Variables|Character|GetMesh))))
  (Variables|Animation|SetMyAnimInstance _asbp_nurse_animation)
  (CallFunction|EventConnectonPhaseChanged))