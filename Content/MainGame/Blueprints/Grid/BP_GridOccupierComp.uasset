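; Actor component that tracks which grid square its owner stands on and flags it as occupied for the turn-phase system.
; It listens to BP_GM's phase-change dispatcher and refreshes on Move, Attack and Turn End.
; Each refresh clears the previous square, then finds the current one through the grid manager using the owner's location.
; The square's MyGridInfo is marked occupied only during Move, leaving it unoccupied in Attack and Turn End.
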(event Custom|Dis_OnPhaseChanged_Event_0
  (params (OldPhase :type EPhase%20Enum :default "PE_None"))
  (switch Utilities|FlowControl|Switch|SwitchonEPhase (Class|SmthTacticalGameModeBase|GetCurrentPhase (Variables|Default|GetAs%20BP%20GM))
    (:PE_Move
      _)
    (:PE_Attack
      _)
    (:PE_TurnEnd
      _))
  (CallFunction|RefreshOccupiedGrid))

(event EventBeginPlay
  (bind _asbp_gm (Utilities|Casting|CastToBP_GM (Game|GetGameMode)))
  (bind _output_get (Variables|Default|SetAs%20BP%20GM _asbp_gm))
  (EventDispatchers|AssignDisonPhaseChanged _output_get (delegate Custom|Dis_OnPhaseChanged_Event_0)))

(event EventTick
  (params (DeltaSeconds :type Float%20%28single-precision%29)))

(fn RefreshOccupiedGrid
  (CallFunction|Clear)
  (bind _asbp_gm (Utilities|Casting|CastToBP_GM (Game|GetGameMode)))
  (bind _output_get (LocalVariables|SetMyGamemode _asbp_gm))
  (bind _returnvalue (Class|SquareGridManager|GetSquareGridbyPosition (Default|GetGridManager _output_get) (Transformation|GetActorLocation (Components|GetOwner))))
  (Utilities|IsValid _returnvalue
    (:Is%20Valid
      (Variables|Default|SetOccupiedGrid _returnvalue)
      (bind _asmy_grid_info (Utilities|Casting|CastToMyGridInfo (Variables|/Script/GridRuntime.Grid|GetGridInfo _returnvalue)))
      (LocalVariables|SetMyGridInfo _asmy_grid_info)
      (switch Utilities|FlowControl|Switch|SwitchonEPhase (Class|SmthTacticalGameModeBase|GetCurrentPhase (LocalVariables|GetMyGamemode))
        (:PE_Move
          (Variables|/Game/MainGame/Blueprints/Grid/MyGridInfo.MyGridInfo_C|SetIsOccupied (LocalVariables|GetMyGridInfo) true))
        (:PE_Attack
          (Variables|/Game/MainGame/Blueprints/Grid/MyGridInfo.MyGridInfo_C|SetIsOccupied (LocalVariables|GetMyGridInfo) false))))))

(fn Clear
  (Utilities|IsValid (Variables|Default|GetOccupiedGrid)
    (:Is%20Valid
      (bind _asmy_grid_info (Utilities|Casting|CastToMyGridInfo (Variables|/Script/GridRuntime.Grid|GetGridInfo (Variables|Default|GetOccupiedGrid))))
      (Variables|/Game/MainGame/Blueprints/Grid/MyGridInfo.MyGridInfo_C|SetIsOccupied _asmy_grid_info false)
      (Variables|Default|SetOccupiedGrid 0))))