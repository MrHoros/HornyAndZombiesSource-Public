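; MyGridInfo is a grid info Blueprint that stores per-cell state for a grid: whether the cell is movable, attackable or occupied.
; Setter functions update each flag and call Dirty to mark the info as changed, and matching getters return the current values.
; The Clear event calls the parent Clear, then resets all three flags to false.
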(event EventClear
  ;[1 1 1] Clear
  (|CallParentFunction)
  (Variables|Default|SetIsMovable false)
  (Variables|Default|SetIsAttackble false)
  (Variables|Default|SetIsOccupied false))

(fn SetMovable
  (params (NewMovable :type Boolean))
  (Variables|Default|SetIsMovable NewMovable)
  (Class|GridInfo|Dirty))

(fn SetAttackable
  (params (NewAttackable :type Boolean))
  (Variables|Default|SetIsAttackble NewAttackable)
  (Class|GridInfo|Dirty))

(fn GetIsMovable
  (return (Variables|Default|GetIsMovable)))

(fn GetIsAttackable
  (return (Variables|Default|GetIsAttackble)))

(fn SetIsOccupied
  (params (IsOccupied :type Boolean))
  (Variables|Default|SetIsOccupied IsOccupied)
  (Class|GridInfo|Dirty))

(fn GetIsOccupied
  (return (Variables|Default|GetIsOccupied)))