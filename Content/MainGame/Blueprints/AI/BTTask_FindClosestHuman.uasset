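; Behavior tree task that finds the human-team character closest to the AI's controlled pawn.
; On execute it casts the pawn to BP_CharacterBase and the game mode to BP_GM, then asks the game mode for the nearest character on the human team index.
; A valid result is written to the ClosestHuman blackboard key and the task succeeds; a failed cast or no result fails it.
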(event EventReceiveExecuteAI
  (params (OwnerController :type AI%20Controller%20Object%20Reference) (ControlledPawn :type Pawn%20Object%20Reference))
  (Variables|Default|SetOwner%20Controller OwnerController)
  (bind _asbp_character_base (Utilities|Casting|CastToBP_CharacterBase ControlledPawn)
    (:then
      (Variables|Default|SetMyCharacter _asbp_character_base)
      (bind _asbp_gm (Utilities|Casting|CastToBP_GM (Game|GetGameMode))
        (:then
          (bind _output_get (Variables|Default|SetMyGamemode _asbp_gm))
          (bind _returnvalue (Class|SmthTacticalGameModeBase|GetClosestCharacterOfTeamIndex _output_get (Default|GetHumanTeamIndex _asbp_gm) (Transformation|GetActorLocation (Variables|Default|GetMyCharacter))))
          (bind _output_get_2 (Variables|Default|SetClosestEnemy _returnvalue))
          (Utilities|IsValid _output_get_2
            (:Is%20Valid
              (AI|Components|Blackboard|SetValueasObject (AI|GetBlackboard (Variables|Default|GetOwner%20Controller)) (Utilities|Name|MakeLiteralName "ClosestHuman") (Variables|Default|GetClosestEnemy))
              (AI|BehaviorTree|FinishExecute true))
            (:Is%20Not%20Valid
              (AI|BehaviorTree|FinishExecute false))))
        (:CastFailed
          (AI|BehaviorTree|FinishExecute false :!label _label))))
    (:CastFailed
      (goto _label))))