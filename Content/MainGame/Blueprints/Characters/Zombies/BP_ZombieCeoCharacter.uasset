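; BP_ZombieCeoCharacter is the CEO zombie character, a child Blueprint that adds its own animation hookup to the parent class.
; On BeginPlay, after the parent logic, it casts the mesh's anim instance to BP_zombie_ceo_animation and caches it.
; UpdateAnimVariables copies the run, death, damaged and attack state variables into that anim instance as floats.
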(event EventBeginPlay
  (|CallParentFunction)
  (bind _asbp_zombie_ceo_animation (Utilities|Casting|CastToBP_zombie_ceo_animation (Components|SkeletalMesh|GetAnimInstance (Variables|Character|GetMesh))))
  (Variables|Animation|SetMyAnimInstance _asbp_zombie_ceo_animation))

(fn ConstructionScript
  (|CallParentFunction))

(fn UpdateAnimVariables
  (Utilities|FlowControl|Sequence
    (:then_0
      (Variables|/Game/MainGame/Mannequin/Animations/Zombies/BP_zombie_ceo_animation.BP_zombie_ceo_animation_C|Setwalk_0 (Variables|Animation|GetMyAnimInstance) (Math|Conversions|ToFloat(Integer) (Variables|Default|GetRunAnimVariable))))
    (:then_1
      (Variables|/Game/MainGame/Mannequin/Animations/Zombies/BP_zombie_ceo_animation.BP_zombie_ceo_animation_C|Setdeath_0 (Variables|Animation|GetMyAnimInstance) (Math|Conversions|ToFloat(Integer) (Variables|Default|GetDeathAnimVariable))))
    (:then_2
      (Variables|/Game/MainGame/Mannequin/Animations/Zombies/BP_zombie_ceo_animation.BP_zombie_ceo_animation_C|Setdamage_0 (Variables|Animation|GetMyAnimInstance) (Math|Conversions|ToFloat(Integer) (Variables|Default|GetDamagedAnimVariable))))
    (:then_3
      (Variables|/Game/MainGame/Mannequin/Animations/Zombies/BP_zombie_ceo_animation.BP_zombie_ceo_animation_C|Setattack_0 (Variables|Animation|GetMyAnimInstance) (Math|Conversions|ToFloat(Integer) (Variables|Default|GetAttackAnimVariable))))))